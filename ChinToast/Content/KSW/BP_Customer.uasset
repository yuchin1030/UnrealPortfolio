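; BP_Customer is a customer actor that shows or hides its timer and recipe widget according to its order state.
; Each Tick, it shows the widget through VisibleWidget when its waiting number is zero and its state is ORDERDELAY.
; Otherwise, it hides the widget when the state is CHECK, and leaves visibility unchanged in all other cases.
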(event `self.ReceiveBeginPlay`)

(event `self.ReceiveTick`
  (params (DeltaSeconds :type "Float (single-precision)"))
  (if (and (== (`self.waitingNum`) 0) (`|EnumEquality` (`self.state`) "ORDERDELAY"))
    (`self.VisibleWidget`)
    (elif (`|EnumEquality` (`self.state`) "CHECK")
      (`SceneComponent.SetVisibility` (`self.TimerRecipeWidget`) false false))))

(fn `UserConstructionScript`)

(fn `VisibleWidget`
  (`SceneComponent.SetVisibility` (`self.TimerRecipeWidget`) true false))