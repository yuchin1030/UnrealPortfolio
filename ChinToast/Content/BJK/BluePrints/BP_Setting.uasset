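; Serving counter actor that takes a wrapped toast order on its tray and resolves it when the player touches the bell.
; BeginPlay caches customers and player; the first wrapping to overlap the box collision loses physics and grab and snaps to the tray socket.
; Tick polls bell overlap for the front waiting customer, checks the recipe and destroys the food.
; Failure or success sets customer flags and effects, with success also adding score.
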(event `self.ReceiveBeginPlay`
  (bind _outactors (`GameplayStatics.GetAllActorsOfClass` "/Game/KSW/BP_Customer.BP_Customer_C"))
  (set `self.Customers` _outactors)
  (bind _asbp_test_player (cast `/Game/BJK/BluePrints/BP_TestPlayer` (`GameplayStatics.GetPlayerPawn` 0)))
  (set `self.PlayerVar` _asbp_test_player))

(event `self.BoxingCol.OnComponentBeginOverlap`
  (params (OverlappedComponent :type "PrimitiveComponent Object Reference") (OtherActor :type "Actor Object Reference") (OtherComp :type "PrimitiveComponent Object Reference") (OtherBodyIndex :type Integer) (bFromSweep :type Boolean) (SweepResult :type "HitResult Structure (by ref)"))
  (if (not (`self.Do once`))
    (set `self.Do once` true)
    (bind _asbp_wrapping (cast `/Game/BJK/BluePrints/BP_Wrapping` OtherActor))
    (`PrimitiveComponent.SetSimulatePhysics` (`/Game/BJK/BluePrints/BP_Wrapping.StaticMesh` _asbp_wrapping) false)
    (`/Game/BJK/BluePrints/BP_Wrapping.DestroyGrab` _asbp_wrapping)
    (`SceneComponent.K2_AttachToComponent` (`Actor.RootComponent` _asbp_wrapping) (`self.Tray`) "TaryS" "SnapToTarget" "SnapToTarget" "SnapToTarget" true)))

(event `self.ReceiveTick`
  (params (DeltaSeconds :type "Float (single-precision)"))
  (bind _playervar (`self.PlayerVar`))
  (bind _wrappingvar (`self.WrappingVar`))
  (bind _wrappingvar_2 (`self.WrappingVar`))
  (bind _returnvalue_location (`KismetMathLibrary.BreakTransform` (`SceneComponent.GetSocketTransform` (`self.Tray`) "A" "RTS_World")))
  (bind _fail (`/Game/BJK/BluePrints/BP_Wrapping.fail` _wrappingvar_2))
  (for _array_element (`self.Customers`)
    (`/Engine/EditorBlueprintResources/StandardMacros.IsValid` _array_element
      (:`Is Valid`
        (if (== (`Customer.waitingNum` _array_element) 0)
          ;[1 1 1] 쟁반 위에 포장상자 및 재료들이 있고, 벨까지 눌러야 삭제됨
          (bind _output_get (set `self.CustomerVar` _array_element))
          (`/Engine/EditorBlueprintResources/StandardMacros.IsValid` _playervar
            (:`Is Valid`
              (if (and (`PrimitiveComponent.IsOverlappingComponent` (`self.ButtonCol`) (`/Game/BJK/BluePrints/BP_TestPlayer.Sphere1` _playervar)) (`self.Do once`) (`|EnumEquality` (`Customer.state` _output_get) "ORDERDELAY"))
                (`/Engine/EditorBlueprintResources/StandardMacros.IsValid` _wrappingvar
                  (:`Is Valid`
                    (`/Game/BJK/BluePrints/BP_Wrapping.CheckRecipe` _wrappingvar)
                    (`/Game/BJK/BluePrints/BP_Wrapping.DestroyFoodAndBox` _wrappingvar) ; 쟁반에 올려지면 포장박스, 재료들 삭제
                    (set `Customer.getfood` true (`self.CustomerVar`))
                    (set `self.isGameOver` true)
                    (`KismetSystemLibrary.PrintString` (`KismetStringLibrary.Conv_BoolToString` _fail))
                    (if _fail
                      (set `Customer.orderSuccess` false (`self.CustomerVar`))
                      (`NiagaraFunctionLibrary.SpawnSystemAtLocation` "/Game/KSW/VFX/NS_Fail.NS_Fail" _returnvalue_location)
                      (set `self.Do once` false :!label _label)
                      (else
                        (`|ExecutionSequence`
                          (:`then_0`
                            (bind _aswbp_timer_recipe (cast `/Game/Yuchin/UI/WBP_Timer_Recipe` (`WidgetComponent.GetWidget` (`/Game/KSW/BP_Customer.TimerRecipeWidget` (`self.CustomerVar`)))))
                            (`/Game/Yuchin/UI/WBP_Timer_Recipe.CheckScore` _aswbp_timer_recipe)
                            (if (>= (`KismetArrayLibrary.Array_Length` (`/Game/BJK/BluePrints/BP_Wrapping.FoodArr` _wrappingvar_2)) 5)
                              (bind _returnvalue (`|SpawnActorFromClass` "/Game/Yuchin/Blueprints/BP_SpawnedPlusScore.BP_SpawnedPlusScore_C" (`KismetMathLibrary.MakeTransform` (-1150.0 -104.0 145.0) (struct) (0.5 0.5 0.5)) "Undefined" "MultiplyWithRoot" null null)) ; 플러스되는 점수 UI 띄우기
                              (`/Game/Yuchin/Blueprints/BP_SpawnedPlusScore.SetScore` _returnvalue (`self.Score`))
                              (set `self.Sum` (+ (`self.Sum`) (`self.Score`)))
                              (`KismetSystemLibrary.Delay` 1.0)))
                          (:`then_1`
                            (`KismetSystemLibrary.PrintString` "Hello" true true (struct :`G` 0.66 :`B` 1.0 :`A` 1.0) 1000.0)
                            (set `Customer.orderSuccess` true (`self.CustomerVar`))
                            (`GameplayStatics.PlaySound2D` "/Game/KSW/sound/success.success" 1.0 1.0 0.0 null null)
                            (`NiagaraFunctionLibrary.SpawnSystemAtLocation` "/Game/KSW/VFX/NS_Bread.NS_Bread" _returnvalue_location)
                            (goto _label)))))))))))))))

(event `self.ButtonCol.OnComponentBeginOverlap`
  (params (OverlappedComponent :type "PrimitiveComponent Object Reference") (OtherActor :type "Actor Object Reference") (OtherComp :type "PrimitiveComponent Object Reference") (OtherBodyIndex :type Integer) (bFromSweep :type Boolean) (SweepResult :type "HitResult Structure (by ref)"))
  (cast `/Game/BJK/BluePrints/BP_TestPlayer` OtherActor)
  (`GameplayStatics.PlaySound2D` "/Game/KSW/sound/bell_Cue.bell_Cue" 1.0 1.0 0.0 null null))

(event `CheckScore`)

(fn `UserConstructionScript`)