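; Baking zone actor that turns a BP_BreadBase left inside its Box into a BP_Bread after a timed delay.
; The finished bread spawns far from the scene, then moves to just above the base's former position after the base is destroyed.
; Overlap exit clears the Bake flag, which gates both the swap and a later delayed destruction of the bread.
; BP_BreadBurn spawning exists but is disconnected.
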(event `self.Box.OnComponentBeginOverlap`
  (params (OverlappedComponent :type "PrimitiveComponent Object Reference") (OtherActor :type "Actor Object Reference") (OtherComp :type "PrimitiveComponent Object Reference") (OtherBodyIndex :type Integer) (bFromSweep :type Boolean) (SweepResult :type "HitResult Structure (by ref)"))
  (bind _asbp_bread_base (cast `/Game/BJK/BluePrints/Food/BP_BreadBase` OtherActor))
  (set `self.Bake` true)
  (`KismetSystemLibrary.Delay` 3.0)
  (if (`self.Bake`)
    (bind _returnvalue_location (`KismetMathLibrary.BreakTransform` (`self.GetTransform` _asbp_bread_base)))
    (set `self.Spawn` (+ (* (`self.GetActorUpVector` _asbp_bread_base) 5.0) _returnvalue_location))
    (bind _returnvalue (`|SpawnActorFromClass` "/Game/BJK/BluePrints/Food/BP_Bread.BP_Bread_C" (`KismetMathLibrary.MakeTransform` (0.0 0.0 10000.0)) "AlwaysSpawn" "MultiplyWithRoot" null null))
    (`self.K2_DestroyActor` OtherActor)
    (`KismetSystemLibrary.Delay` 0.2)
    (`self.K2_SetActorLocation` _returnvalue (`self.Spawn`) false false)
    (if (`self.Bake`)
      (`KismetSystemLibrary.Delay` 3.0)
      (`self.K2_DestroyActor` _returnvalue))))

(event `self.Box.OnComponentEndOverlap`
  (params (OverlappedComponent :type "PrimitiveComponent Object Reference") (OtherActor :type "Actor Object Reference") (OtherComp :type "PrimitiveComponent Object Reference") (OtherBodyIndex :type Integer))
  (cast `/Game/BJK/BluePrints/Food/BP_BreadBase` OtherActor)
  (set `self.Bake` false)
  (set `self.Burn` false))

(fn `UserConstructionScript`)