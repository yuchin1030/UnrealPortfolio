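; BP_Lettuce is a lettuce food actor that can be grabbed and placed on a BP_Wrapping.
; When its Box overlaps the wrapping's CheckF component, it destroys its grab component if valid.
; Overlapping any other actor type starts a 16-second delay, after which the lettuce destroys itself unless IsAttachLettuce is set.
; This graph only reads that flag and never sets it.
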(event `self.Box.OnComponentBeginOverlap`
  (params (OverlappedComponent :type "PrimitiveComponent Object Reference") (OtherActor :type "Actor Object Reference") (OtherComp :type "PrimitiveComponent Object Reference") (OtherBodyIndex :type Integer) (bFromSweep :type Boolean) (SweepResult :type "HitResult Structure (by ref)"))
  (bind _asbp_wrapping (cast `/Game/BJK/BluePrints/BP_Wrapping` OtherActor)
    (:`then`
      (if (== (`/Game/BJK/BluePrints/BP_Wrapping.CheckF` _asbp_wrapping) OtherComp)
        (`/Engine/EditorBlueprintResources/StandardMacros.IsValid` null
          (:`Is Valid`
            (`ActorComponent.K2_DestroyComponent` (`self.GrabComponent1`))))))
    (:`CastFailed`
      (`KismetSystemLibrary.Delay` 16.0)
      (if (not (`self.isAttachLettuce`))
        (`self.K2_DestroyActor`)))))

(fn `UserConstructionScript`)