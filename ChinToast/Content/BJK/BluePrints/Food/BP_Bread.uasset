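; BP_Bread is a grabbable bread food actor that can be wrapped, burned or cleaned up.
; When its Box overlaps a BP_Wrapping's CheckF component, it destroys its grab component so it can no longer be grabbed.
; Overlapping any other actor starts a 16-second delay, after which it destroys itself unless IsAttachBread is set.
; MakeBurn, gated by IsBurning, replaces it with a BP_BreadBurn spawned high up and teleported just above it.
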(event `self.Box.OnComponentBeginOverlap`
  (params (OverlappedComponent :type "PrimitiveComponent Object Reference") (OtherActor :type "Actor Object Reference") (OtherComp :type "PrimitiveComponent Object Reference") (OtherBodyIndex :type Integer) (bFromSweep :type Boolean) (SweepResult :type "HitResult Structure (by ref)"))
  (bind _asbp_wrapping (cast `/Game/BJK/BluePrints/BP_Wrapping` OtherActor)
    (:`then`
      (if (== (`/Game/BJK/BluePrints/BP_Wrapping.CheckF` _asbp_wrapping) OtherComp)
        (`ActorComponent.K2_DestroyComponent` (`self.GrabComponent1`))))
    (:`CastFailed`
      (`KismetSystemLibrary.Delay` 16.0)
      (if (not (`self.isAttachBread`))
        (`self.K2_DestroyActor`)))))

(fn `MakeBurn`
  (if (`self.isBurning`)
    (bind _returnvalue (`|SpawnActorFromClass` "/Game/BJK/BluePrints/Food/BP_BreadBurn.BP_BreadBurn_C" (`KismetMathLibrary.MakeTransform` (0.0 0.0 1000.0)) "Undefined" "MultiplyWithRoot" null null))
    (`self.K2_SetActorLocation` _returnvalue (+ (`self.K2_GetActorLocation`) (0.0 0.0 10.0)) false true)
    (`self.K2_DestroyActor`)))

(fn `UserConstructionScript`)