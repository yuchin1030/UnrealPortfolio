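; BP_Wrapping is a wrapping actor that collects sandwich ingredients and checks them against the Recipe actor.
; CheckF overlaps, ignoring player, setting, board and knife actors, snap items onto sockets A to E in order, while CheckFood logs each ingredient's name and flags it attached.
; CheckRecipe compares that ordered list with the recipe, setting Fail on a mismatch.
; Tick polls the customer once-gated, destroying food and wrapper on CHECK state.
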(event `self.ReceiveBeginPlay`
  (bind _outactors (`GameplayStatics.GetAllActorsOfClass` "/Game/KSW/Recipe.Recipe_C"))
  (set `self.RecipeVar` (`|GetArrayItem` _outactors))
  (bind _returnvalue (`GameplayStatics.GetActorOfClass` "/Game/KSW/BP_Customer.BP_Customer_C"))
  (set `self.customer` _returnvalue))

(event `self.CheckF.OnComponentBeginOverlap`
  (params (OverlappedComponent :type "PrimitiveComponent Object Reference") (OtherActor :type "Actor Object Reference") (OtherComp :type "PrimitiveComponent Object Reference") (OtherBodyIndex :type Integer) (bFromSweep :type Boolean) (SweepResult :type "HitResult Structure (by ref)"))
  (cast `/Game/BJK/BluePrints/BP_TestPlayer` OtherActor
    (:`CastFailed`
      (cast `/Game/BJK/BluePrints/BP_Setting` OtherActor
        (:`CastFailed`
          (cast `/Game/BJK/BluePrints/cuttingboard/BP_cuttingBoard` OtherActor
            (:`CastFailed`
              (cast `/Game/BJK/BluePrints/cuttingboard/BP_Knife` OtherActor
                (:`CastFailed`
                  (switch `int` (`self.isAttach`)
                    (:`0`
                      (`/Engine/EditorBlueprintResources/StandardMacros.DoOnce` false
                        (:`Completed`
                          (`self.K2_AttachToActor` OtherActor self "A" "SnapToTarget" "SnapToTarget" "SnapToTarget" true)
                          (bind _result (`/Engine/EditorBlueprintResources/StandardMacros.IncrementInt` (`self.isAttach`))
                            (:`  `
                              (set `self.isAttach` _result)
                              (`self.CheckFood` OtherActor))))))
                    (:`1`
                      (`/Engine/EditorBlueprintResources/StandardMacros.DoOnce` false
                        (:`Completed`
                          (`self.K2_AttachToActor` OtherActor self "B" "SnapToTarget" "SnapToTarget" "SnapToTarget" true)
                          (bind _result_2 (`/Engine/EditorBlueprintResources/StandardMacros.IncrementInt` (`self.isAttach`))
                            (:`  `
                              (set `self.isAttach` _result_2)
                              (`self.CheckFood` OtherActor))))))
                    (:`2`
                      (`/Engine/EditorBlueprintResources/StandardMacros.DoOnce` false
                        (:`Completed`
                          (`self.K2_AttachToActor` OtherActor self "C" "SnapToTarget" "SnapToTarget" "SnapToTarget" true)
                          (bind _result_3 (`/Engine/EditorBlueprintResources/StandardMacros.IncrementInt` (`self.isAttach`))
                            (:`  `
                              (set `self.isAttach` _result_3)
                              (`self.CheckFood` OtherActor))))))
                    (:`3`
                      (`/Engine/EditorBlueprintResources/StandardMacros.DoOnce` false
                        (:`Completed`
                          (`self.K2_AttachToActor` OtherActor self "D" "SnapToTarget" "SnapToTarget" "SnapToTarget" true)
                          (bind _result_4 (`/Engine/EditorBlueprintResources/StandardMacros.IncrementInt` (`self.isAttach`))
                            (:`  `
                              (set `self.isAttach` _result_4)
                              (`self.CheckFood` OtherActor))))))
                    (:`4`
                      (`/Engine/EditorBlueprintResources/StandardMacros.DoOnce` false
                        (:`Completed`
                          (`self.K2_AttachToActor` OtherActor self "E" "SnapToTarget" "SnapToTarget" "SnapToTarget" true)
                          (bind _result_5 (`/Engine/EditorBlueprintResources/StandardMacros.IncrementInt` (`self.isAttach`))
                            (:`  `
                              (set `self.isAttach` _result_5)
                              (`self.CheckFood` OtherActor))))))))))))))))

(event `CheckRecipe`
  (for _index (range 1 6)
    (bind _returnvalue (`KismetStringLibrary.EqualEqual_StrStr` (`|GetArrayItem` (`ChinToastRecipe.makedRecipe` (`self.RecipeVar`)) _index) (`|GetArrayItem` (`self.MakingFood`) (- _index 1))))
    (`KismetSystemLibrary.PrintString` (`KismetStringLibrary.Conv_BoolToString` _returnvalue) true true (struct :`G` 0.66 :`B` 1.0 :`A` 1.0) 10.0)
    (if _returnvalue
      (`KismetSystemLibrary.PrintString` "fail is false")
      (else
        (set `self.fail` true)
        (`KismetSystemLibrary.PrintString` "fail is true")
        (break)))))

(event `self.ReceiveTick`
  (params (DeltaSeconds :type "Float (single-precision)"))
  (`/Engine/EditorBlueprintResources/StandardMacros.DoOnce` false
    (:`Completed`
      (if (`|EnumEquality` (`Customer.state` (`self.customer`)) "CHECK")
        (`self.DestroyFoodAndBox`)))))

(event `DestroyFoodAndBox`
  (bind _foodarr (`self.FoodArr`))
  (for (_ _array_index) _foodarr
    (bind _output (`|GetArrayItem` _foodarr _array_index))
    (`/Engine/EditorBlueprintResources/StandardMacros.IsValid` _output
      (:`Is Valid`
        (`self.K2_DestroyActor` _output)
        (`KismetSystemLibrary.Delay` 1.0 :!label _label)
        (`KismetArrayLibrary.Array_Clear` (`self.FoodArr`))
        (`self.K2_DestroyActor`)
        (`KismetSystemLibrary.PrintString` "dkanrjsk"))))
  (goto _label))

(fn `CheckFood`
  (params (NewParam :type "Actor Object Reference"))
  (bind _foodarr (`self.FoodArr`))
  (bind _asbp_bread (cast `/Game/BJK/BluePrints/Food/BP_Bread` NewParam)
    (:`then`
      (`KismetArrayLibrary.Array_Add` (`self.MakingFood`) "Bread")
      (`KismetArrayLibrary.Array_Add` _foodarr _asbp_bread)
      (set `/Game/BJK/BluePrints/Food/BP_Bread.isAttachBread` true _asbp_bread))
    (:`CastFailed`
      (bind _asbp_tomato (cast `/Game/BJK/BluePrints/Food/BP_Tomato` NewParam)
        (:`then`
          (`KismetArrayLibrary.Array_Add` (`self.MakingFood`) "Tomato")
          (`KismetArrayLibrary.Array_Add` _foodarr _asbp_tomato)
          (set `/Game/BJK/BluePrints/Food/BP_Tomato.isAttachTomato` true _asbp_tomato))
        (:`CastFailed`
          (bind _asbp_ham (cast `/Game/BJK/BluePrints/Food/BP_Ham` NewParam)
            (:`then`
              (`KismetArrayLibrary.Array_Add` (`self.MakingFood`) "Hams")
              (`KismetArrayLibrary.Array_Add` _foodarr _asbp_ham)
              (set `/Game/BJK/BluePrints/Food/BP_Ham.isAttachHam` true _asbp_ham))
            (:`CastFailed`
              (bind _asbp_chesse (cast `/Game/BJK/BluePrints/Food/BP_Chesse` NewParam)
                (:`then`
                  (`KismetArrayLibrary.Array_Add` (`self.MakingFood`) "Cheese")
                  (`KismetArrayLibrary.Array_Add` _foodarr _asbp_chesse)
                  (set `/Game/BJK/BluePrints/Food/BP_Chesse.isAttachChesse` true _asbp_chesse))
                (:`CastFailed`
                  (bind _asbp_lettuce (cast `/Game/BJK/BluePrints/Food/BP_Lettuce` NewParam))
                  (`KismetArrayLibrary.Array_Add` (`self.MakingFood`) "Lettuce")
                  (`KismetArrayLibrary.Array_Add` _foodarr _asbp_lettuce)
                  (set `/Game/BJK/BluePrints/Food/BP_Lettuce.isAttachLettuce` true _asbp_lettuce))))))))))

(fn `DestroyGrab`
  (`ActorComponent.K2_DestroyComponent` (`self.GrabComponent1`)))

(fn `UserConstructionScript`)