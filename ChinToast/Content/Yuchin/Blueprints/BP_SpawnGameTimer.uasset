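; Countdown game timer actor that ends the round by showing the final result and destroying every BP_Customer.
; BeginPlay caches the BP_SpawnFinalResult actor and the UI_GameTimer from its widget component.
; Tick uses a Delay as a one-second gate to decrement minutes and seconds, with no guard against repeating the end step at zero.
; ClockAnim, not called here, plays a warning sound and looping seconds animation while its counter lasts.
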(event `self.ReceiveBeginPlay`
  (`|ExecutionSequence`
    (:`then_0`
      (bind _outactors (`GameplayStatics.GetAllActorsOfClass` "/Game/Yuchin/Blueprints/BP_SpawnFinalResult.BP_SpawnFinalResult_C"))
      (set `self.SpawnFinalResultVar` (`|GetArrayItem` _outactors)))
    (:`then_1`
      (bind _asui_game_timer (cast `/Game/Yuchin/UI/UI_GameTimer` (`WidgetComponent.GetWidget` (`self.Widget`))))
      (set `self.As UI Game Timer` _asui_game_timer))))

(event `self.ReceiveTick`
  (params (DeltaSeconds :type "Float (single-precision)"))
  (`KismetSystemLibrary.Delay` 1.0)
  (if (== (`self.Seconds`) 0)
    (if (== (`self.Minutes`) 0)
      (`/Game/Yuchin/Blueprints/BP_SpawnFinalResult.ShowFinalResult` (`self.SpawnFinalResultVar`))
      (bind _outactors (`GameplayStatics.GetAllActorsOfClass` "/Game/KSW/BP_Customer.BP_Customer_C"))
      (for _array_element _outactors
        (`/Engine/EditorBlueprintResources/StandardMacros.IsValid` _array_element
          (:`Is Valid`
            (`self.K2_DestroyActor` _array_element)
            (bind _rootcomponent (`Actor.RootComponent` _array_element))
            (`/Engine/EditorBlueprintResources/StandardMacros.IsValid` _rootcomponent
              (:`Is Valid`
                (`ActorComponent.K2_DestroyComponent` _rootcomponent))))))
      (else
        (set `self.Seconds` 59)
        (set `self.Minutes` (- (`self.Minutes`) 1))))
    (else
      (set `self.Seconds` (- (`self.Seconds`) 1)))))

(fn `ClockAnim`
  (bind _animtimercnt (`self.animTimerCnt`))
  (bind _as_ui_game_timer (`self.As UI Game Timer`))
  (if (> _animtimercnt 0)
    (bind _result (`/Engine/EditorBlueprintResources/StandardMacros.DecrementInt` _animtimercnt)
      (:`  `
        (set `self.animTimerCnt` _result)
        (`GameplayStatics.PlaySound2D` "/Game/KSW/sound/warning-sound_Cue.warning-sound_Cue" 1.0 1.0 0.0 null null)
        (`UserWidget.PlayAnimation` _as_ui_game_timer (`/Game/Yuchin/UI/UI_GameTimer.SecondsANim` _as_ui_game_timer) 0.0 0 "Forward" 1.0 false)))))

(fn `UserConstructionScript`)