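; Table cover actor that plays the panel-flip cutscene between the table puzzle and the rear table switch.
; The construction script orders left and right panels into two arrays.
; FlipStart replays a timeline with a counter as a pseudo-loop, rotating each pair, correcting its height, then playing a sound and applying yellow or blue glowing material by mesh shape.
; Afterwards it teleports the player to MovePos, sets their view and enables the rear switch.
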(event `self.ReceiveBeginPlay`
  ;[1 1 1] 이전 퍼즐인 테이블 퍼즐과 다음 상호작용인 뒷편 스위치를 변수로 선언
  (bind _outactors (`GameplayStatics.GetAllActorsOfClass` "/Game/BoxesLike/BluePrints/Box2-2/BP_TablePuzzle.BP_TablePuzzle_C"))
  (set `self.TablePuzzle` (`|GetArrayItem` _outactors))
  (bind _outactors_2 (`GameplayStatics.GetAllActorsOfClass` "/Game/BoxesLike/BluePrints/Box2-2/BP_RearTableSwitch.BP_RearTableSwitch_C"))
  (set `self.RearTableSwitch` (`|GetArrayItem` _outactors_2)))

(event `FlipStart`
  (bind (_movepos_location _movepos_rotation) (`KismetMathLibrary.BreakTransform` (`self.MovePos`)))
  (bind _output (`|GetArrayItem` (`self.LeftPanelList`) (`self.LoopCount`)))
  (bind _output_2 (`|GetArrayItem` (`self.RightPanelList`) (`self.LoopCount`)))
  ;[1 1 1] 판넬 회전 연출구간. 타임라인은 For문과 함께 사용할 수 없으므로,  변수 LoopCount를 이용하여 유사 루프문을 만들었다. 배열의 갯수만큼 반복하고 종료된다
  ; 레벨시퀸스는 레벨블루프린트에서만 저장되므로, FlipStart판정은 레벨블루프린트에서 실시한다.
  (`KismetSystemLibrary.Delay` 2.0)
  (bind (_direction _value) (`Timeline|FlipTimeLine` :!label _label)
    (:`Update`
      (`self.FlipMove` _output _value)
      (`self.FlipMove` _output_2 _value))
    (:`Finished`
      (`GameplayStatics.PlaySound2D` "/Game/BoxesLike/Sound/SE/Choi/SEC_gun_hit_1_Cue.SEC_gun_hit_1_Cue" 1.0 1.0 0.0 null null)
      (`self.FlipMatChange` _output true)
      (`self.FlipMatChange` _output_2)
      (bind _output_get (set `self.LoopCount` (+ (`self.LoopCount`) 1)))
      (if (< _output_get 14)
        (goto _label :!via `PlayFromStart`)
        (else
          ;[1 1 1] 테이블 패널이 다 뒤집히면 플레이어 캐릭터를 테이블 뒤로 이동시키고, 테이블을 바라보게 한다.
          (`self.K2_TeleportTo` :`self` (`GameplayStatics.GetPlayerCharacter` 0) :`DestLocation` (`KismetMathLibrary.TransformLocation` (`self.GetTransform`) _movepos_location))
          (`Controller.SetControlRotation` (`GameplayStatics.GetPlayerController` 0) _movepos_rotation)
          (set `/Game/BoxesLike/BluePrints/Box2-2/BP_RearTableSwitch.FlipComplete` true (`self.RearTableSwitch`)))))))

(fn `FlipMatChange`
  (params (FlipPanel :type "StaticMeshComponent Object Reference") (LisTandRisF :type Boolean))
  (bind _staticmesh (`StaticMeshComponent.StaticMesh` (`local.FlipPanel`)))
  (bind _staticmesh_2 (`StaticMeshComponent.StaticMesh` (`local.FlipPanel`)))
  (bind _returnvalue (or (== _staticmesh "/Game/BoxesLike/StaticMesh/Box2-2/SM_FlipBoardBL.SM_FlipBoardBL") (== _staticmesh "/Game/BoxesLike/StaticMesh/Box2-2/SM_FlipBoardBR.SM_FlipBoardBR") (== _staticmesh "/Game/BoxesLike/StaticMesh/Box2-2/SM_FlipBoardTL.SM_FlipBoardTL") (== _staticmesh "/Game/BoxesLike/StaticMesh/Box2-2/SM_FlipBoardTR.SM_FlipBoardTR")))
  (bind _returnvalue_2 (or (== _staticmesh_2 "/Game/BoxesLike/StaticMesh/Box2-2/SM_FlipBoardLR.SM_FlipBoardLR") (== _staticmesh_2 "/Game/BoxesLike/StaticMesh/Box2-2/SM_FlipBoardTB.SM_FlipBoardTB")))
  ;[1 1 1] 뒤집힌 패널의 가운데 금 메테리얼을 빛나는 메테리얼로 변경한다. 좌우의 색이 다르고, 패널 형태마다 금 메테리얼의 위치가 달라 Branch문으로 구분한다.
  (if LisTandRisF
    (if _returnvalue_2
      (`PrimitiveComponent.SetMaterial` (`local.FlipPanel`) 3 "/Game/BoxesLike/Materials/M_YellowLightMetal.M_YellowLightMetal")
      (elif _returnvalue
        (`PrimitiveComponent.SetMaterial` (`local.FlipPanel`) 2 "/Game/BoxesLike/Materials/M_YellowLightMetal.M_YellowLightMetal")
        (else
          (`PrimitiveComponent.SetMaterial` (`local.FlipPanel`) 0 "/Game/BoxesLike/Materials/M_YellowLightMetal.M_YellowLightMetal"))))
    (elif _returnvalue_2
      (`PrimitiveComponent.SetMaterial` (`local.FlipPanel`) 3 "/Game/BoxesLike/Materials/M_BlueLightMetal.M_BlueLightMetal")
      (elif _returnvalue
        (`PrimitiveComponent.SetMaterial` (`local.FlipPanel`) 2 "/Game/BoxesLike/Materials/M_BlueLightMetal.M_BlueLightMetal")
        (else
          (`PrimitiveComponent.SetMaterial` (`local.FlipPanel`) 0 "/Game/BoxesLike/Materials/M_BlueLightMetal.M_BlueLightMetal"))))))

(fn `FlipMove`
  (params (FlipPanel :type "StaticMeshComponent Object Reference") (TimelineValue :type "Float (double-precision)"))
  (locals (MoveZ :type "Float (double-precision)" :default 2.0) (PanelStartRotation :type "Rotator Structure" :default (struct)))
  (bind _staticmesh (`StaticMeshComponent.StaticMesh` FlipPanel))
  (bind (_relativelocation_x _relativelocation_y) (`KismetMathLibrary.BreakVector` (`SceneComponent.RelativeLocation` FlipPanel)))
  ;[1 1 1] 뒤집혀져서 Z축 위치가 틀어져 있으므로, Rotation과 함께 Z축 값도 보정한다.
  (bind _output_get (set `local.PanelStartRotation` (`SceneComponent.RelativeRotation` FlipPanel)))
  (if (or (== _staticmesh "/Game/BoxesLike/StaticMesh/Box2-2/SM_FlipBoardLL.SM_FlipBoardLL") (== _staticmesh "/Game/BoxesLike/StaticMesh/Box2-2/SM_FlipBoardRR.SM_FlipBoardRR"))
    (set `local.MoveZ` 2.5) ; 마지막 패널은 크기가 커서 더 보정한다
    (else
      (set `local.MoveZ` 2.0)))
  (`SceneComponent.K2_SetRelativeLocationAndRotation` FlipPanel (`KismetMathLibrary.MakeVector` _relativelocation_x _relativelocation_y (`local.MoveZ`)) (`KismetMathLibrary.RLerp` _output_get (struct) TimelineValue) false false))

(fn `UserConstructionScript`
  ;[1 1 1] 배열에 패널 초기화 실시. 순서대로 좌우를 구분하여 입력한다
  (`|ExecutionSequence`
    (:`then_0`
      (`KismetArrayLibrary.Array_Set` (`self.LeftPanelList`) 0 (`self.SM_OverTurnPanelLStart`))
      (`KismetArrayLibrary.Array_Set` (`self.LeftPanelList`) 1 (`self.SM_OverTurnPanelL1`))
      (`KismetArrayLibrary.Array_Set` (`self.LeftPanelList`) 2 (`self.SM_OverTurnPanelL2`))
      (`KismetArrayLibrary.Array_Set` (`self.LeftPanelList`) 3 (`self.SM_OverTurnPanelL3`))
      (`KismetArrayLibrary.Array_Set` (`self.LeftPanelList`) 4 (`self.SM_OverTurnPanelL4`))
      (`KismetArrayLibrary.Array_Set` (`self.LeftPanelList`) 5 (`self.SM_OverTurnPanelL5`))
      (`KismetArrayLibrary.Array_Set` (`self.LeftPanelList`) 6 (`self.SM_OverTurnPanelL6`))
      (`KismetArrayLibrary.Array_Set` (`self.LeftPanelList`) 7 (`self.SM_OverTurnPanelL7`))
      (`KismetArrayLibrary.Array_Set` (`self.LeftPanelList`) 8 (`self.SM_OverTurnPanelL8`))
      (`KismetArrayLibrary.Array_Set` (`self.LeftPanelList`) 9 (`self.SM_OverTurnPanelL9`))
      (`KismetArrayLibrary.Array_Set` (`self.LeftPanelList`) 10 (`self.SM_OverTurnPanelL10`))
      (`KismetArrayLibrary.Array_Set` (`self.LeftPanelList`) 11 (`self.SM_OverTurnPanelL11`))
      (`KismetArrayLibrary.Array_Set` (`self.LeftPanelList`) 12 (`self.SM_OverTurnPanelL12`))
      (`KismetArrayLibrary.Array_Set` (`self.LeftPanelList`) 13 (`self.SM_OverTurnPanelLEnd`)))
    (:`then_1`
      (`KismetArrayLibrary.Array_Set` (`self.RightPanelList`) 0 (`self.SM_OverTurnPanelRStart`))
      (`KismetArrayLibrary.Array_Set` (`self.RightPanelList`) 1 (`self.SM_OverTurnPanelR1`))
      (`KismetArrayLibrary.Array_Set` (`self.RightPanelList`) 2 (`self.SM_OverTurnPanelR2`))
      (`KismetArrayLibrary.Array_Set` (`self.RightPanelList`) 3 (`self.SM_OverTurnPanelR3`))
      (`KismetArrayLibrary.Array_Set` (`self.RightPanelList`) 4 (`self.SM_OverTurnPanelR4`))
      (`KismetArrayLibrary.Array_Set` (`self.RightPanelList`) 5 (`self.SM_OverTurnPanelR5`))
      (`KismetArrayLibrary.Array_Set` (`self.RightPanelList`) 6 (`self.SM_OverTurnPanelR6`))
      (`KismetArrayLibrary.Array_Set` (`self.RightPanelList`) 7 (`self.SM_OverTurnPanelR7`))
      (`KismetArrayLibrary.Array_Set` (`self.RightPanelList`) 8 (`self.SM_OverTurnPanelR8`))
      (`KismetArrayLibrary.Array_Set` (`self.RightPanelList`) 9 (`self.SM_OverTurnPanelR9`))
      (`KismetArrayLibrary.Array_Set` (`self.RightPanelList`) 10 (`self.SM_OverTurnPanelR10`))
      (`KismetArrayLibrary.Array_Set` (`self.RightPanelList`) 11 (`self.SM_OverTurnPanelR11`))
      (`KismetArrayLibrary.Array_Set` (`self.RightPanelList`) 12 (`self.SM_OverTurnPanelR12`))
      (`KismetArrayLibrary.Array_Set` (`self.RightPanelList`) 13 (`self.SM_OverTurnPanelREnd`)))))