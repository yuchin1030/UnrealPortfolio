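; BP_GunBox is a puzzle box that hides a screwdriver and a power cell.
; A one-shot rear button pops out a drawer handle and shows the screwdriver, then input passes to the box for mouse-drag drawer pulling.
; TopCoverOpen swings four cover pieces open via timeline, then raises the power cell, which copies the rotation of an invisible spinning RotatePoint.
; The construction script finds both items by ItemID and caches a gear-set actor.
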(event `self.ReceiveBeginPlay`
  ;[1 1 1] 배터리만 회전시키기 위해 형태가 존재하지 않는 RotatePoint만 돌리게 한다.
  (`MovementComponent.SetUpdatedComponent` (`self.RotatingMovement`) (`self.RotatePoint`)))

(event `self.ReceiveTick`
  (params (DeltaSeconds :type "Float (single-precision)"))
  (bind _powercell (`self.PowerCell`))
  ;[1 1 1] 떠오른 배터리가 천천히 회전한다.
  (`/Engine/EditorBlueprintResources/StandardMacros.IsValid` _powercell
    (:`Is Valid`
      (`self.K2_SetActorRotation` _powercell (`SceneComponent.RelativeRotation` (`self.RotatePoint`)) false))))

(event `self.RearButtonCol.OnClicked`
  (params (TouchedComponent :type "PrimitiveComponent Object Reference") (ButtonPressed :type "Key Structure"))
  (bind (_relativelocation_x _relativelocation_y _relativelocation_z) (`KismetMathLibrary.BreakVector` (`SceneComponent.RelativeLocation` (`self.RearButtonTrue`))))
  (bind (_relativelocation_x_2 _relativelocation_y_2 _relativelocation_z_2) (`KismetMathLibrary.BreakVector` (`SceneComponent.RelativeLocation` (`self.RearDrawerHandle`))))
  ;[1 1 1] 뒷면 버튼을 누르면 버튼이 눌리고 서랍 핸들이 튀어나온다
  (`/Engine/EditorBlueprintResources/StandardMacros.DoOnce` false
    (:`Completed`
      (`self.DisableInput` (`GameplayStatics.GetPlayerPawn` 0) (`GameplayStatics.GetPlayerController` 0))
      (`GameplayStatics.PlaySound2D` "/Game/BoxesLike/Sound/SE/Choi/SEC_gun_hit_1_Cue.SEC_gun_hit_1_Cue" 1.0 1.0 0.0 null null)
      (set `self.RearButtonStartX` _relativelocation_x)
      (bind (_direction _movingrate) (`Timeline|ButtonPush`)
        (:`Update`
          (`SceneComponent.K2_SetRelativeLocation` (`self.RearButtonTrue`) (`KismetMathLibrary.MakeVector` (+ (* _movingrate -5.0) (`self.RearButtonStartX`)) _relativelocation_y _relativelocation_z) false false))
        (:`Finished`
          (`GameplayStatics.PlaySound2D` "/Game/BoxesLike/Sound/SE/Choi/SEC_kitchen_drawer_open_3_Cue.SEC_kitchen_drawer_open_3_Cue" 1.0 1.0 0.0 null null)
          (set `self.RearHandleStartX` _relativelocation_x_2)
          (bind (_direction_2 _movingrate_2) (`Timeline|MoveHandle`)
            (:`Update`
              (`SceneComponent.K2_SetRelativeLocation` (`self.RearDrawerHandle`) (`KismetMathLibrary.MakeVector` (+ (* _movingrate_2 -5.5) (`self.RearHandleStartX`)) _relativelocation_y_2 _relativelocation_z_2) false false))
            (:`Finished`
              (`self.EnableInput` (`GameplayStatics.GetPlayerPawn` 0) (`GameplayStatics.GetPlayerController` 0))
              (`StaticMeshComponent.SetStaticMesh` (`/Game/BoxesLike/BluePrints/TestBoxBP/BP_ItemActor.StaticMesh` (`self.Driver`)) "/Game/BoxesLike/StaticMesh/Box2-2/SM_ScrewDriver.SM_ScrewDriver"))))))))

(event `/Game/BoxesLike/BPInterface/BlockMoving.Block Moving`
  (params (Mover :type "Pawn Object Reference") (ClickPoint :type "Vector Structure") (LookingComponentPoint :type "PrimitiveComponent Object Reference"))
  (bind _returnvalue (`GameplayStatics.GetPlayerController` 0))
  ;[1 1 1] 아이템 상세 확인 시작/종료 부분. 상세 확인을 시작하면 플레이어 캐릭터에 있던 컨트롤을 생성된 이 액터로 옮긴다.
  (if (== LookingComponentPoint (`self.RearHandleColl`))
    (`self.DisableInput` Mover _returnvalue)
    (`self.EnableInput` _returnvalue)))

(event `Key|LeftMouseButton`
  (params (Key :type "Key Structure"))
  (bind _returnvalue (`GameplayStatics.GetPlayerController` 0))
  ;[1 1 1] 아이템 상세 확인 시작/종료 부분. 상세 확인을 시작하면 플레이어 캐릭터에 있던 컨트롤을 생성된 이 액터로 옮긴다.
  (:`Released`
    (`self.DisableInput` _returnvalue :!label _label)
    (`self.EnableInput` (stale `/Game/BoxesLike/BPInterface/BlockMoving.Block Moving` Mover) _returnvalue)))

(event `StopMoving`
  ;[1 1 1] 아이템 상세 확인 시작/종료 부분. 상세 확인을 시작하면 플레이어 캐릭터에 있던 컨트롤을 생성된 이 액터로 옮긴다.
  (goto _label))

(event `InputAxisKey|MouseY`
  (params (AxisValue :type "Float (single-precision)"))
  (bind _returnvalue (* AxisValue -3.0))
  (bind (_returnvalue_x _returnvalue_y _returnvalue_z) (`KismetMathLibrary.BreakVector` (`self.K2_GetActorLocation` (`self.Driver`))))
  (bind _relativelocation_x (`KismetMathLibrary.BreakVector` (`SceneComponent.RelativeLocation` (`self.RearDrawer`))))
  (bind (_relativelocation_x_2 _relativelocation_y _relativelocation_z) (`KismetMathLibrary.BreakVector` (`SceneComponent.RelativeLocation` (`self.RearDrawer`))))
  (bind _returnvalue_2 (+ _returnvalue _relativelocation_x_2))
  ;[1 1 1] 마우스를 드래그하면 이 스태틱 매쉬가 이동한다. 원하는 축/방향에 맞춰서 X/Y , XYZ 연결을 조정
  (if (and (< AxisValue 0.0) (< _relativelocation_x 98.0) (`PlayerController.IsInputKeyDown` (`GameplayStatics.GetPlayerController` 0) "LeftMouseButton"))
    (`SceneComponent.K2_SetRelativeLocation` (`self.RearDrawer`) (`KismetMathLibrary.MakeVector` _returnvalue_2 _relativelocation_y _relativelocation_z) false false)
    (if (> _returnvalue_2 98.0)
      (`SceneComponent.K2_SetRelativeLocation` (`self.RearDrawer`) (`KismetMathLibrary.MakeVector` 98.0 _relativelocation_y _relativelocation_z) false false)
      (`GameplayStatics.PlaySound2D` "/Game/BoxesLike/Sound/SE/Choi/SEC_hole_puncher_1_Cue.SEC_hole_puncher_1_Cue" 1.0 1.0 0.0 null null)
      (`self.StopMoving`)
      (else
        (`self.K2_SetActorLocation` (`self.Driver`) (`KismetMathLibrary.MakeVector` (+ (/ _returnvalue 2.0) _returnvalue_x) _returnvalue_y _returnvalue_z) false false)))))

(event `TopCoverOpen`
  (bind _powercell (`self.PowerCell`))
  (bind (_powercellstartloc_x _powercellstartloc_y _powercellstartloc_z) (`KismetMathLibrary.BreakVector` (`self.PowerCellStartLoc`)))
  ;[1 1 1] 상단 커버 열림 연출
  (`/Engine/EditorBlueprintResources/StandardMacros.DoOnce` false
    (:`Completed`
      (`GameplayStatics.PlaySound2D` "/Game/BoxesLike/Sound/SE/Choi/SEC_sci-fi_door_2_Cue.SEC_sci-fi_door_2_Cue" 1.0 1.0 0.0 null null)
      (bind (_direction _value) (`Timeline|TopOpen`)
        (:`Update`
          (`self.TopOpener` _value) ; 커버 4개가 한꺼번에 열린다.
        )
        (:`Finished`
          (`StaticMeshComponent.SetStaticMesh` (`/Game/BoxesLike/BluePrints/TestBoxBP/BP_ItemActor.StaticMesh` _powercell) "/Game/BoxesLike/Assets/PowerCellEc/EC_Power_Cell.EC_Power_Cell")
          (set `self.PowerCellStartLoc` (`self.K2_GetActorLocation` _powercell))
          (`ActorComponent.Activate` (`self.Niagara`) false)
          (`GameplayStatics.PlaySound2D` "/Game/BoxesLike/Sound/SE/Choi/SEC_floating_Cue.SEC_floating_Cue" 1.0 1.0 0.0 null null)
          (`ActorComponent.Activate` (`self.RotatingMovement`) false)
          (bind (_direction_2 _value_2) (`Timeline|PowerCellUp`)
            (:`Update`
              (`self.K2_SetActorLocation` (`self.PowerCell`) (`KismetMathLibrary.MakeVector` _powercellstartloc_x _powercellstartloc_y (+ _powercellstartloc_z (* _value_2 40.0))) false false))))))))

(fn `TopOpener`
  (params (TimeLineValue :type "Float (double-precision)"))
  (locals (RotateValue :type "Rotator Structure" :default (struct)) (Start1 :type "Rotator Structure" :default (struct)) (Start2 :type "Rotator Structure" :default (struct)) (Start3 :type "Rotator Structure" :default (struct)) (Start4 :type "Rotator Structure" :default (struct)))
  (bind (_start1_roll _start1_pitch _start1_yaw) (`KismetMathLibrary.BreakRotator` (`local.Start1`)))
  (bind (_start2_roll _start2_pitch _start2_yaw) (`KismetMathLibrary.BreakRotator` (`local.Start2`)))
  (bind (_start3_roll _start3_pitch _start3_yaw) (`KismetMathLibrary.BreakRotator` (`local.Start3`)))
  (bind (_start4_roll _start4_pitch _start4_yaw) (`KismetMathLibrary.BreakRotator` (`local.Start4`)))
  (`|ExecutionSequence`
    (:`then_0`
      ;[1 1 1] 모두 자기 자신 위치에서 X방향으로 -90도 회전
      (bind _output_get (set `local.Start1` (`SceneComponent.RelativeRotation` (`self.SM_TopGlobePiece1`))))
      (`SceneComponent.K2_SetRelativeRotation` (`self.SM_TopGlobePiece1`) (`KismetMathLibrary.RLerp` _output_get (`KismetMathLibrary.MakeRotator` -90.0 _start1_pitch _start1_yaw) (`local.TimeLineValue`) true) false false))
    (:`then_1`
      (bind _output_get_2 (set `local.Start2` (`SceneComponent.RelativeRotation` (`self.SM_TopGlobePiece2`))))
      (`SceneComponent.K2_SetRelativeRotation` (`self.SM_TopGlobePiece2`) (`KismetMathLibrary.RLerp` _output_get_2 (`KismetMathLibrary.MakeRotator` -90.0 _start2_pitch _start2_yaw) (`local.TimeLineValue`) true) false false))
    (:`then_2`
      (bind _output_get_3 (set `local.Start3` (`SceneComponent.RelativeRotation` (`self.SM_TopGlobePiece3`))))
      (`SceneComponent.K2_SetRelativeRotation` (`self.SM_TopGlobePiece3`) (`KismetMathLibrary.RLerp` _output_get_3 (`KismetMathLibrary.MakeRotator` -90.0 _start3_pitch _start3_yaw) (`local.TimeLineValue`) true) false false))
    (:`then_3`
      (bind _output_get_4 (set `local.Start4` (`SceneComponent.RelativeRotation` (`self.SM_TopGlobePiece4`))))
      (`SceneComponent.K2_SetRelativeRotation` (`self.SM_TopGlobePiece4`) (`KismetMathLibrary.RLerp` _output_get_4 (`KismetMathLibrary.MakeRotator` -90.0 _start4_pitch _start4_yaw) (`local.TimeLineValue`) true) false false))))

(fn `UserConstructionScript`
  ;[1 1 1] 드라이버와 파워셀, 우측 톱니바퀴 블루프린트를 변수로 저장
  (`|ExecutionSequence`
    (:`then_0`
      (bind _outactors (`GameplayStatics.GetAllActorsOfClass` "/Game/BoxesLike/BluePrints/TestBoxBP/BP_ItemActor.BP_ItemActor_C"))
      (for _array_element _outactors
        (if (== (`/Game/BoxesLike/BluePrints/TestBoxBP/BP_ItemActor.ItemID` _array_element) 24)
          (bind _output_get (set `self.Driver` _array_element))
          (`StaticMeshComponent.SetStaticMesh` (`/Game/BoxesLike/BluePrints/TestBoxBP/BP_ItemActor.StaticMesh` _output_get) null)
          (elif (== (`/Game/BoxesLike/BluePrints/TestBoxBP/BP_ItemActor.ItemID` _array_element) 29)
            (bind _output_get_2 (set `self.PowerCell` _array_element))
            (`StaticMeshComponent.SetStaticMesh` (`/Game/BoxesLike/BluePrints/TestBoxBP/BP_ItemActor.StaticMesh` _output_get_2) null)))))
    (:`then_1`
      (bind _outactors_2 (`GameplayStatics.GetAllActorsOfClass` "/Game/BoxesLike/BluePrints/Box2-2/BP_LeftGearSet.BP_LeftGearSet_C"))
      (set `self.LeftGearSet` (`|GetArrayItem` _outactors_2)))))