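; BP_ClickButton is a test clickable button actor that triggers a 90-degree rotation on a ClickAndRotate actor.
; It finds the first ClickAndRotate on BeginPlay, enables mouse click events, and calls Rotate90 when its MiddleButton component is clicked.
; The PiecesRotating event takes input from a Rotator and gives it to the button, and releasing the left mouse button hands it back.
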(event `self.ReceiveBeginPlay`
  (bind _outactors (`GameplayStatics.GetAllActorsOfClass` "/Game/BoxesLike/BluePrints/TestBoxBP/ClickAndRotate.ClickAndRotate_C"))
  (set `self.CR_Var` (`|GetArrayItem` _outactors))
  (set `PlayerController.bEnableClickEvents` true (`GameplayStatics.GetPlayerController` 0)))

(event `/Game/BoxesLike/BPInterface/BlockRotating90.PiecesRotating`
  (params (Rotator :type "Pawn Object Reference") (`Click Point` :type "Vector Structure"))
  (bind _returnvalue (`GameplayStatics.GetPlayerController` 0))
  (`self.DisableInput` Rotator _returnvalue)
  (`self.EnableInput` _returnvalue))

(event `Key|LeftMouseButton`
  (params (Key :type "Key Structure"))
  (bind _returnvalue (`GameplayStatics.GetPlayerController` 0))
  (:`Released`
    (`self.DisableInput` _returnvalue)
    (`self.EnableInput` (stale `/Game/BoxesLike/BPInterface/BlockRotating90.PiecesRotating` Rotator) _returnvalue)))

(event `self.MiddleButton.OnClicked`
  (params (TouchedComponent :type "PrimitiveComponent Object Reference") (ButtonPressed :type "Key Structure"))
  (`KismetSystemLibrary.PrintString` "Click YEs")
  (`/Game/BoxesLike/BluePrints/TestBoxBP/ClickAndRotate.Rotate90` (`self.CR_Var`)))

(fn `UserConstructionScript`)