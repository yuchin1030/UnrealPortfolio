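; BP_OrderEvent2 is a test actor for ordered click events, acting only once BP_OrderEvent1 has its TestFlag set.
; On BeginPlay it caches the first BP_OrderEvent1 found in the level as its prerequisite.
; Clicking its Box then toggles its own TestFlag, deactivating the particle system when the flag turns on and activating it when the flag turns off.
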(event `self.ReceiveBeginPlay`
  (bind _outactors (`GameplayStatics.GetAllActorsOfClass` "/Game/BoxesLike/BluePrints/TestBoxBP/BP_OrderEvent1.BP_OrderEvent1_C"))
  (set `self.BeforeEventActor` (`|GetArrayItem` _outactors)))

(event `self.Box.OnClicked`
  (params (TouchedComponent :type "PrimitiveComponent Object Reference") (ButtonPressed :type "Key Structure"))
  (bind _particlesystem (`self.ParticleSystem`))
  (if (`/Game/BoxesLike/BluePrints/TestBoxBP/BP_OrderEvent1.TestFlag` (`self.BeforeEventActor`))
    (if (`self.TestFlag`)
      (set `self.TestFlag` false)
      (`ActorComponent.Activate` _particlesystem false)
      (else
        (set `self.TestFlag` true)
        (`ActorComponent.Deactivate` _particlesystem)))))

(fn `UserConstructionScript`)