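; Item inspection actor that displays a given mesh for the player to examine and rotate by mouse drag.
; The construction script applies InspectItemShape to the mesh, and StartInspect moves input from the Inspector to this actor.
; While the left button is held, mouse axes set mesh yaw and pitch from the actor rotation.
; Right click returns input to the Inspector and calls EndInspectMouse on the first-person character.
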(event `/Game/BoxesLike/BPInterface/StartInspect.StartInspect`
  (params (Inspector :type "Pawn Object Reference"))
  (bind _returnvalue (`GameplayStatics.GetPlayerController` 0))
  ;[1 1 1] 아이템 상세 확인 시작/종료 부분. 상세 확인을 시작하면 플레이어 캐릭터에 있던 컨트롤을 생성된 이 액터로 옮긴다.
  (`self.DisableInput` Inspector _returnvalue)
  (`self.EnableInput` _returnvalue))

(event `Key|RightMouseButton`
  (params (Key :type "Key Structure"))
  (bind _returnvalue (`GameplayStatics.GetPlayerController` 0))
  ;[1 1 1] 아이템 상세 확인 시작/종료 부분. 상세 확인을 시작하면 플레이어 캐릭터에 있던 컨트롤을 생성된 이 액터로 옮긴다.
  (:`Pressed`
    (`self.DisableInput` _returnvalue)
    (`self.EnableInput` (stale `/Game/BoxesLike/BPInterface/StartInspect.StartInspect` Inspector) _returnvalue)
    (bind _asbp_first_person_character (cast `/Game/FirstPerson/Blueprints/BP_FirstPersonCharacter` (`GameplayStatics.GetPlayerCharacter` 0)))
    (`/Game/FirstPerson/Blueprints/BP_FirstPersonCharacter.EndInspectMouse` _asbp_first_person_character)))

(event `InputAxisKey|MouseX`
  (params (AxisValue :type "Float (single-precision)"))
  ;[1 1 1] 마우스를 드래그하면 이 스태틱 매쉬가 회전한다.
  (if (`PlayerController.IsInputKeyDown` (`GameplayStatics.GetPlayerController` 0) "LeftMouseButton")
    (`SceneComponent.K2_SetRelativeRotation` (`self.StaticMesh`) (`KismetMathLibrary.ComposeRotators` (`self.K2_GetActorRotation`) (`KismetMathLibrary.MakeRotator` 0.0 0.0 (* AxisValue -1.0))) false false)))

(event `InputAxisKey|MouseY`
  (params (AxisValue :type "Float (single-precision)"))
  ;[1 1 1] 마우스를 드래그하면 이 스태틱 매쉬가 회전한다.
  (if (`PlayerController.IsInputKeyDown` (`GameplayStatics.GetPlayerController` 0) "LeftMouseButton")
    (`SceneComponent.K2_SetRelativeRotation` (`self.StaticMesh`) (`KismetMathLibrary.ComposeRotators` (`self.K2_GetActorRotation`) (`KismetMathLibrary.MakeRotator` 0.0 (* AxisValue -1.0))) false false)))

(fn `UserConstructionScript`
  ;[1 1 1] 생성될때 입력받은 스태틱매쉬로 겉모습 생성
  (`StaticMeshComponent.SetStaticMesh` (`self.StaticMesh`) (`self.InspectItemShape`)))