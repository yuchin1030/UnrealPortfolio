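; Test box Blueprint with two static meshes that rotate in opposite directions, triggered by a mouse click.
; BeginPlay binds RotatingMovement to StaticMesh, and clicking that mesh plays a Timeline that drives its yaw.
; When the Timeline finishes, it activates RotatingMovement to rotate the mesh.
; Every Tick, StaticMesh1 takes the negated relative rotation of StaticMesh, mirroring its motion.
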(event `self.ReceiveBeginPlay`
  (`MovementComponent.SetUpdatedComponent` (`self.RotatingMovement`) (`self.StaticMesh`)))

(event `self.ReceiveTick`
  (params (DeltaSeconds :type "Float (single-precision)"))
  (`SceneComponent.K2_SetRelativeRotation` (`self.StaticMesh1`) (* (`SceneComponent.RelativeRotation` (`self.StaticMesh`)) -1.0) false false))

(event `self.StaticMesh.OnClicked`
  (params (TouchedComponent :type "PrimitiveComponent Object Reference") (ButtonPressed :type "Key Structure"))
  (bind (_direction _newtrack_0) (`Timeline|Timeline`)
    (:`Update`
      (`SceneComponent.K2_SetRelativeRotation` (`self.StaticMesh`) (`KismetMathLibrary.MakeRotator` 0.0 0.0 (* _newtrack_0 120.0)) false false))
    (:`Finished`
      (`ActorComponent.Activate` (`self.RotatingMovement`) false))))

(fn `UserConstructionScript`)