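; ClickAndRotate is a test Blueprint that turns its root component about the pitch axis in successive steps each time its Rotate90 event is called.
; An Order counter selects one of four timelines, whose negated TLRotate90 track drives relative pitch, and each update sets Order to the next step.
; The fourth step wraps Order to zero and, after a short Delay started from the timeline update, resets the rotation to zero.
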(event `self.ReceiveBeginPlay`)

(event `Rotate90`
  (switch `int` (`self.Order`)
    (:`0`
      (bind (_direction _tl_rotate90) (`Timeline|Timeline_0` :!via `PlayFromStart`)
        (:`Update`
          (`SceneComponent.K2_SetRelativeRotation` (`self.DefaultSceneRoot`) (`KismetMathLibrary.MakeRotator` 0.0 (* _tl_rotate90 -1.0)) false false)
          (set `self.Order` 1))))
    (:`1`
      (bind (_direction_2 _tl_rotate90_2) (`Timeline|Timeline` :!via `PlayFromStart`)
        (:`Update`
          (`SceneComponent.K2_SetRelativeRotation` (`self.DefaultSceneRoot`) (`KismetMathLibrary.MakeRotator` 0.0 (* _tl_rotate90_2 -1.0)) false false)
          (set `self.Order` 2))))
    (:`2`
      (bind (_direction_3 _tl_rotate90_3) (`Timeline|Timeline_1` :!via `PlayFromStart`)
        (:`Update`
          (`SceneComponent.K2_SetRelativeRotation` (`self.DefaultSceneRoot`) (`KismetMathLibrary.MakeRotator` 0.0 (* _tl_rotate90_3 -1.0)) false false)
          (set `self.Order` 3))))
    (:`3`
      (bind (_direction_4 _tl_rotate90_4) (`Timeline|Timeline_2` :!via `PlayFromStart`)
        (:`Update`
          (`SceneComponent.K2_SetRelativeRotation` (`self.DefaultSceneRoot`) (`KismetMathLibrary.MakeRotator` 0.0 (* _tl_rotate90_4 -1.0)) false false)
          (set `self.Order` 0)
          (`KismetSystemLibrary.Delay` 1.0)
          (`SceneComponent.K2_SetRelativeRotation` :`self` (`self.DefaultSceneRoot`)))))))

(fn `UserConstructionScript`)