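; Last-box puzzle piece where a compass with indicator lights guides the search for a pendant on BP_LastBoxGlobe.
; Using an item reveals and slides in the compass, then stops the globe; a separate event slides away the glass wireframe.
; While mouse input is detected, Tick greens lights outward from Light7 as squared XY pendant-to-compass distance shrinks.
; Overlap triggers clear sounds, orange light and particles once, then sets CanLastSQ.
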(event `self.ReceiveBeginPlay`
  (`SceneComponent.SetVisibility` (`self.CompassAnim`) false false)
  (`SceneComponent.SetVisibility` (`self.Light1`) false false)
  (`SceneComponent.SetVisibility` (`self.Light2`) false false)
  (`SceneComponent.SetVisibility` (`self.Light3`) false false)
  (`SceneComponent.SetVisibility` (`self.Light4`) false false)
  (`SceneComponent.SetVisibility` (`self.Light5`) false false)
  (`SceneComponent.SetVisibility` (`self.Light6`) false false)
  (`SceneComponent.SetVisibility` (`self.Light7`) false false)
  (`SceneComponent.SetVisibility` (`self.Light8`) false false)
  (`SceneComponent.SetVisibility` (`self.Light9`) false false)
  (`SceneComponent.SetVisibility` (`self.Light10`) false false)
  (`SceneComponent.SetVisibility` (`self.Light11`) false false)
  (`SceneComponent.SetVisibility` (`self.Light12`) false false)
  (`SceneComponent.SetVisibility` (`self.OrangeLight`) false false)
  (bind _outactors (`GameplayStatics.GetAllActorsOfClass` "/Game/BoxesLike/BluePrints/RealBoxYuchin/BP_LastBoxGlobe.BP_LastBoxGlobe_C"))
  (set `self.LastBxVar` (`|GetArrayItem` _outactors))
  (bind _outactors_2 (`GameplayStatics.GetAllActorsOfClass` "/Game/BoxesLike/BluePrints/RealBoxYuchin/BP_ItemShip.BP_ItemShip_C"))
  (set `self.ShipVar` (`|GetArrayItem` _outactors_2)))

(event `CompassAnimStart`
  (`SceneComponent.SetVisibility` (`self.CompassAnim`) true false)
  (`SceneComponent.SetVisibility` (`self.Light1`) true false)
  (`SceneComponent.SetVisibility` (`self.Light2`) true false)
  (`SceneComponent.SetVisibility` (`self.Light3`) true false)
  (`SceneComponent.SetVisibility` (`self.Light4`) true false)
  (`SceneComponent.SetVisibility` (`self.Light5`) true false)
  (`SceneComponent.SetVisibility` (`self.Light6`) true false)
  (`SceneComponent.SetVisibility` (`self.Light7`) true false)
  (`SceneComponent.SetVisibility` (`self.Light8`) true false)
  (`SceneComponent.SetVisibility` (`self.Light9`) true false)
  (`SceneComponent.SetVisibility` (`self.Light10`) true false)
  (`SceneComponent.SetVisibility` (`self.Light11`) true false)
  (`SceneComponent.SetVisibility` (`self.Light12`) true false)
  (`GameplayStatics.PlaySound2D` "/Game/BoxesLike/Sound/SE/Yuchin/LastB_CompassAnim.LastB_CompassAnim" 1.0 1.0 0.0 null null)
  (bind (_direction _cp) (`Timeline|Compass`)
    (:`Update`
      (`SceneComponent.K2_SetRelativeLocation` (`self.CompassAnim`) (`KismetMathLibrary.MakeVector` 0.0 _cp) false false)
      (`KismetSystemLibrary.Delay` 1.5)
      (`/Game/BoxesLike/BluePrints/RealBoxYuchin/BP_LastBoxGlobe.StopGlobe` (`self.LastBxVar`))
      (set `self.isGlobeStopped` true))))

(event `Destroy GlassWF`
  (`GameplayStatics.PlaySound2D` "/Game/BoxesLike/Sound/SE/Yuchin/LastB_GlassSliceDisappear_Cue.LastB_GlassSliceDisappear_Cue" 1.0 1.0 0.0 null null)
  (bind (_direction _wf) (`Timeline|GlassWF`)
    (:`Update`
      (`SceneComponent.K2_SetRelativeLocation` (`self.GlassWireframe`) (`KismetMathLibrary.MakeVector` 1.0 _wf 1.0) false false))))

(event `FindPendant`)

(event `self.ReceiveTick`
  (params (DeltaSeconds :type "Float (single-precision)"))
  (bind _light7 (`self.Light7`))
  (bind _light6 (`self.Light6`))
  (bind _light5 (`self.Light5`))
  (bind _light4 (`self.Light4`))
  (bind _light3 (`self.Light3`))
  (bind _light2 (`self.Light2`))
  (bind _light1 (`self.Light1`))
  (bind (_returnvalue_x _returnvalue_y) (`KismetMathLibrary.BreakVector` (`SceneComponent.K2_GetComponentLocation` (`self.CompassCollision`))))
  (bind (_returnvalue_x_2 _returnvalue_y_2) (`KismetMathLibrary.BreakVector` (`SceneComponent.K2_GetComponentLocation` (`/Game/BoxesLike/BluePrints/RealBoxYuchin/BP_LastBoxGlobe.PendantCollision` (`self.LastBxVar`)))))
  ;[1 1 1] 펜던트 찾기
  (if (and (`self.isGlobeStopped`) (`/Game/BoxesLike/BluePrints/RealBoxYuchin/BP_LastBoxGlobe.isMouseDetected` (`self.LastBxVar`)))
    (set `self.Distance` (+ (`KismetMathLibrary.Square` (- _returnvalue_x _returnvalue_x_2)) (`KismetMathLibrary.Square` (- _returnvalue_y _returnvalue_y_2))))
    (if (<= (`self.Distance`) 1500.0)
      (`PrimitiveComponent.SetMaterial` _light7 0 "/Game/BoxesLike/Levels/_GENERATED/Yuchin/chaos-emeralds/source/GameCube_-_Sonic_Adventure_DX_Directors_Cut_-_Chaos_Emeralds/EmeraldGreen.EmeraldGreen")
      (else
        (`PrimitiveComponent.SetMaterial` _light7 0 "/Game/BoxesLike/Levels/_GENERATED/Yuchin/chaos-emeralds/source/GameCube_-_Sonic_Adventure_DX_Directors_Cut_-_Chaos_Emeralds/EmeraldRed.EmeraldRed")))
    (if (<= (`self.Distance`) 1200.0)
      (`PrimitiveComponent.SetMaterial` _light6 0 "/Game/BoxesLike/Levels/_GENERATED/Yuchin/chaos-emeralds/source/GameCube_-_Sonic_Adventure_DX_Directors_Cut_-_Chaos_Emeralds/EmeraldGreen.EmeraldGreen")
      (`PrimitiveComponent.SetMaterial` (`self.Light8`) 0 "/Game/BoxesLike/Levels/_GENERATED/Yuchin/chaos-emeralds/source/GameCube_-_Sonic_Adventure_DX_Directors_Cut_-_Chaos_Emeralds/EmeraldGreen.EmeraldGreen")
      (else
        (`PrimitiveComponent.SetMaterial` _light6 0 "/Game/BoxesLike/Levels/_GENERATED/Yuchin/chaos-emeralds/source/GameCube_-_Sonic_Adventure_DX_Directors_Cut_-_Chaos_Emeralds/EmeraldRed.EmeraldRed")
        (`PrimitiveComponent.SetMaterial` (`self.Light8`) 0 "/Game/BoxesLike/Levels/_GENERATED/Yuchin/chaos-emeralds/source/GameCube_-_Sonic_Adventure_DX_Directors_Cut_-_Chaos_Emeralds/EmeraldRed.EmeraldRed")))
    (if (<= (`self.Distance`) 900.0)
      (`PrimitiveComponent.SetMaterial` _light5 0 "/Game/BoxesLike/Levels/_GENERATED/Yuchin/chaos-emeralds/source/GameCube_-_Sonic_Adventure_DX_Directors_Cut_-_Chaos_Emeralds/EmeraldGreen.EmeraldGreen")
      (`PrimitiveComponent.SetMaterial` (`self.Light9`) 0 "/Game/BoxesLike/Levels/_GENERATED/Yuchin/chaos-emeralds/source/GameCube_-_Sonic_Adventure_DX_Directors_Cut_-_Chaos_Emeralds/EmeraldGreen.EmeraldGreen")
      (else
        (`PrimitiveComponent.SetMaterial` _light5 0 "/Game/BoxesLike/Levels/_GENERATED/Yuchin/chaos-emeralds/source/GameCube_-_Sonic_Adventure_DX_Directors_Cut_-_Chaos_Emeralds/EmeraldRed.EmeraldRed")
        (`PrimitiveComponent.SetMaterial` (`self.Light9`) 0 "/Game/BoxesLike/Levels/_GENERATED/Yuchin/chaos-emeralds/source/GameCube_-_Sonic_Adventure_DX_Directors_Cut_-_Chaos_Emeralds/EmeraldRed.EmeraldRed")))
    (if (<= (`self.Distance`) 600.0)
      (`PrimitiveComponent.SetMaterial` _light4 0 "/Game/BoxesLike/Levels/_GENERATED/Yuchin/chaos-emeralds/source/GameCube_-_Sonic_Adventure_DX_Directors_Cut_-_Chaos_Emeralds/EmeraldGreen.EmeraldGreen")
      (`PrimitiveComponent.SetMaterial` (`self.Light10`) 0 "/Game/BoxesLike/Levels/_GENERATED/Yuchin/chaos-emeralds/source/GameCube_-_Sonic_Adventure_DX_Directors_Cut_-_Chaos_Emeralds/EmeraldGreen.EmeraldGreen")
      (else
        (`PrimitiveComponent.SetMaterial` _light4 0 "/Game/BoxesLike/Levels/_GENERATED/Yuchin/chaos-emeralds/source/GameCube_-_Sonic_Adventure_DX_Directors_Cut_-_Chaos_Emeralds/EmeraldRed.EmeraldRed")
        (`PrimitiveComponent.SetMaterial` (`self.Light10`) 0 "/Game/BoxesLike/Levels/_GENERATED/Yuchin/chaos-emeralds/source/GameCube_-_Sonic_Adventure_DX_Directors_Cut_-_Chaos_Emeralds/EmeraldRed.EmeraldRed")))
    (if (<= (`self.Distance`) 300.0)
      (`PrimitiveComponent.SetMaterial` _light3 0 "/Game/BoxesLike/Levels/_GENERATED/Yuchin/chaos-emeralds/source/GameCube_-_Sonic_Adventure_DX_Directors_Cut_-_Chaos_Emeralds/EmeraldGreen.EmeraldGreen")
      (`PrimitiveComponent.SetMaterial` (`self.Light11`) 0 "/Game/BoxesLike/Levels/_GENERATED/Yuchin/chaos-emeralds/source/GameCube_-_Sonic_Adventure_DX_Directors_Cut_-_Chaos_Emeralds/EmeraldGreen.EmeraldGreen")
      (else
        (`PrimitiveComponent.SetMaterial` _light3 0 "/Game/BoxesLike/Levels/_GENERATED/Yuchin/chaos-emeralds/source/GameCube_-_Sonic_Adventure_DX_Directors_Cut_-_Chaos_Emeralds/EmeraldRed.EmeraldRed")
        (`PrimitiveComponent.SetMaterial` (`self.Light11`) 0 "/Game/BoxesLike/Levels/_GENERATED/Yuchin/chaos-emeralds/source/GameCube_-_Sonic_Adventure_DX_Directors_Cut_-_Chaos_Emeralds/EmeraldRed.EmeraldRed")))
    (if (<= (`self.Distance`) 100.0)
      (`PrimitiveComponent.SetMaterial` _light2 0 "/Game/BoxesLike/Levels/_GENERATED/Yuchin/chaos-emeralds/source/GameCube_-_Sonic_Adventure_DX_Directors_Cut_-_Chaos_Emeralds/EmeraldGreen.EmeraldGreen")
      (`PrimitiveComponent.SetMaterial` (`self.Light12`) 0 "/Game/BoxesLike/Levels/_GENERATED/Yuchin/chaos-emeralds/source/GameCube_-_Sonic_Adventure_DX_Directors_Cut_-_Chaos_Emeralds/EmeraldGreen.EmeraldGreen")
      (else
        (`PrimitiveComponent.SetMaterial` _light2 0 "/Game/BoxesLike/Levels/_GENERATED/Yuchin/chaos-emeralds/source/GameCube_-_Sonic_Adventure_DX_Directors_Cut_-_Chaos_Emeralds/EmeraldRed.EmeraldRed")
        (`PrimitiveComponent.SetMaterial` (`self.Light12`) 0 "/Game/BoxesLike/Levels/_GENERATED/Yuchin/chaos-emeralds/source/GameCube_-_Sonic_Adventure_DX_Directors_Cut_-_Chaos_Emeralds/EmeraldRed.EmeraldRed")))
    (if (<= (`self.Distance`) 1.0)
      (`PrimitiveComponent.SetMaterial` _light1 0 "/Game/BoxesLike/Levels/_GENERATED/Yuchin/chaos-emeralds/source/GameCube_-_Sonic_Adventure_DX_Directors_Cut_-_Chaos_Emeralds/EmeraldGreen.EmeraldGreen")
      (else
        (`PrimitiveComponent.SetMaterial` _light1 0 "/Game/BoxesLike/Levels/_GENERATED/Yuchin/chaos-emeralds/source/GameCube_-_Sonic_Adventure_DX_Directors_Cut_-_Chaos_Emeralds/EmeraldRed.EmeraldRed")))
    (if (`PrimitiveComponent.IsOverlappingComponent` (`/Game/BoxesLike/BluePrints/RealBoxYuchin/BP_LastBoxGlobe.PendantCollision` (`self.LastBxVar`)) (`self.CompassCollision`))
      (`/Engine/EditorBlueprintResources/StandardMacros.DoOnce` false
        (:`Completed`
          (`GameplayStatics.PlaySound2D` "/Game/BoxesLike/Sound/SE/Yuchin/LastB_Clear_Cue.LastB_Clear_Cue" 1.0 1.0 0.0 null null)
          (`SceneComponent.SetVisibility` (`self.OrangeLight`) true false)
          (`GameplayStatics.PlaySound2D` "/Game/BoxesLike/Sound/SE/Yuchin/LastB_ClearAfterLight_Cue.LastB_ClearAfterLight_Cue" 1.0 1.0 0.0 null null)
          (bind (_direction _ol) (`Timeline|OrangeLighting`)
            (:`Update`
              (`SceneComponent.K2_SetRelativeLocation` (`self.OrangeLight`) (`KismetMathLibrary.MakeVector` 0.0 _ol) false false)
              (`KismetSystemLibrary.Delay` 2.0)
              (`ActorComponent.Activate` (`self.NS_Particle`) false)
              (set `self.CanLastSQ` true))))))))

(event `self.CompassAnim.OnClicked`
  (params (TouchedComponent :type "PrimitiveComponent Object Reference") (ButtonPressed :type "Key Structure")))

(fn `ItemUsingPoint`
  (params (ItemID :type Integer))
  (returns (ItsUsed :type Boolean))
  (bind _returnvalue (== ItemID (`self.NeedItemID`)))
  (set `self.isItemUsed` _returnvalue)
  (`self.CompassAnimStart`)
  (return _returnvalue))

(fn `UserConstructionScript`)