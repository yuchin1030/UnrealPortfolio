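; Fourth puzzle box, where the player drags two wheels to line up inner pieces and open the doors.
; BlockMoving hands input from the Mover to the box until mouse release, while MouseY turns the grabbed wheel and its linked piece.
; When both pieces sit within set pitch windows, chained timelines retract the wheels and open the doors.
; Separately, Tick lights each target overlapped by any collision sphere, without affecting the solve check.
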(event `self.ReceiveBeginPlay`
  (`SceneComponent.SetVisibility` (`self.Target1`) false false)
  (`SceneComponent.SetVisibility` (`self.Target2`) false false)
  (`SceneComponent.SetVisibility` (`self.Target3`) false false)
  (`SceneComponent.SetVisibility` (`self.Target4`) false false)
  (`SceneComponent.SetVisibility` (`self.DiffTarget`) false false)
  (`SceneComponent.SetVisibility` (`self.Light1`) false false)
  (`SceneComponent.SetVisibility` (`self.Light2`) false false)
  (`SceneComponent.SetVisibility` (`self.Light3`) false false)
  (`SceneComponent.SetVisibility` (`self.Light4`) false false)
  (`SceneComponent.SetVisibility` (`self.LightDiffT`) false false))

(event `/Game/BoxesLike/BPInterface/BlockMoving.Block Moving`
  (params (Mover :type "Pawn Object Reference") (ClickPoint :type "Vector Structure") (LookingComponentPoint :type "PrimitiveComponent Object Reference"))
  (bind _returnvalue (`GameplayStatics.GetPlayerController` 0))
  ;[1 1 1] 플레이어 캐릭터에 있던 컨트롤을 생성된 이 액터로 옮긴다.
  (if (or (== LookingComponentPoint (`self.LeftWheel`)) (== LookingComponentPoint (`self.RightWheel`)))
    (set `self.LookingComponentPoint` LookingComponentPoint)
    (`self.DisableInput` Mover _returnvalue)
    (`self.EnableInput` _returnvalue)))

(event `Key|LeftMouseButton`
  (params (Key :type "Key Structure"))
  (bind _returnvalue (`GameplayStatics.GetPlayerController` 0))
  ;[1 1 1] 플레이어 캐릭터에 있던 컨트롤을 생성된 이 액터로 옮긴다.
  (:`Released`
    (`self.DisableInput` _returnvalue)
    (`self.EnableInput` (stale `/Game/BoxesLike/BPInterface/BlockMoving.Block Moving` Mover) _returnvalue)))

(event `Lighting`
  ;[1 1 1] Target 5개 불빛 들어옴
  (`SceneComponent.SetVisibility` (`self.Target1`) true false)
  (`SceneComponent.SetVisibility` (`self.Target2`) true false)
  (`SceneComponent.SetVisibility` (`self.Target3`) true false)
  (`SceneComponent.SetVisibility` (`self.Target4`) true false)
  (`SceneComponent.SetVisibility` (`self.DiffTarget`) true false))

(event `InputAxisKey|MouseY`
  (params (AxisValue :type "Float (single-precision)"))
  (bind _returnvalue (* AxisValue -0.75))
  (bind (_relativerotation_roll _relativerotation_pitch) (`KismetMathLibrary.BreakRotator` (`SceneComponent.RelativeRotation` (`self.LeftInteract`))))
  (bind (_relativerotation_roll_2 _relativerotation_pitch_2 _relativerotation_yaw) (`KismetMathLibrary.BreakRotator` (`SceneComponent.RelativeRotation` (`self.RightWheel`))))
  (bind (_relativerotation_roll_3 _relativerotation_pitch_3 _relativerotation_yaw_2) (`KismetMathLibrary.BreakRotator` (`SceneComponent.RelativeRotation` (`self.LeftWheel`))))
  (bind (_relativerotation_roll_4 _relativerotation_pitch_4) (`KismetMathLibrary.BreakRotator` (`SceneComponent.RelativeRotation` (`self.Middle`))))
  ;[1 1 1] 물레방아 드래그 회전
  (if (`PlayerController.IsInputKeyDown` (`GameplayStatics.GetPlayerController` 0) "LeftMouseButton")
    (if (and (`self.isWheelAct`) (== (`self.LookingComponentPoint`) (`self.LeftWheel`)))
      (`SceneComponent.K2_SetRelativeRotation` (`self.LeftWheel`) (`KismetMathLibrary.MakeRotator` (+ _relativerotation_roll_3 _returnvalue) _relativerotation_pitch_3 _relativerotation_yaw_2) false false)
      (`SceneComponent.K2_AddLocalRotation` (`self.LeftInteract`) (`KismetMathLibrary.MakeRotator` 0.0 0.0 _returnvalue) false false)
      (if (and (and (>= _relativerotation_pitch 87.0) (<= _relativerotation_pitch 92.0)) (and (>= _relativerotation_pitch_4 -75.0) (<= _relativerotation_pitch_4 -70.0))) :!label _label
        (set `self.isWheelAct` false)
        (`KismetSystemLibrary.Delay` 1.0)
        (`GameplayStatics.PlaySound2D` "/Game/BoxesLike/Sound/SE/Yuchin/FourthB_WheelDisappear_Cue.FourthB_WheelDisappear_Cue" 1.0 1.0 0.0 null null)
        (bind (_direction _lwh) (`Timeline|HideLW`)
          (:`Update`
            (`SceneComponent.K2_SetRelativeLocation` (`self.LeftWheel`) (`KismetMathLibrary.MakeVector` _lwh) false false)
            (bind (_direction_2 _rwh) (`Timeline|HideRW`)
              (:`Update`
                (`SceneComponent.K2_SetRelativeLocation` (`self.RightWheel`) (`KismetMathLibrary.MakeVector` _rwh) false false)
                (`KismetSystemLibrary.Delay` 1.0)
                (bind (_direction_3 _ldo4) (`Timeline|OpenLD`)
                  (:`Update`
                    (`SceneComponent.K2_SetRelativeRotation` (`self.LeftDoor`) (`KismetMathLibrary.MakeRotator` 0.0 0.0 _ldo4) false false)
                    (bind (_direction_4 _rdo4) (`Timeline|OpenRD`)
                      (:`Update`
                        (`SceneComponent.K2_SetRelativeRotation` (`self.RightDoor`) (`KismetMathLibrary.MakeRotator` 0.0 0.0 _rdo4) false false))))
                  (:`Finished`
                    (`GameplayStatics.PlaySound2D` "/Game/BoxesLike/Sound/SE/Yuchin/FourthB_DoorOpen_Cue.FourthB_DoorOpen_Cue" 1.0 1.0 0.0 null null))))))))
      (elif (and (`self.isWheelAct`) (== (`self.LookingComponentPoint`) (`self.RightWheel`)))
        (`SceneComponent.K2_SetRelativeRotation` (`self.RightWheel`) (`KismetMathLibrary.MakeRotator` (+ _returnvalue _relativerotation_roll_2) _relativerotation_pitch_2 _relativerotation_yaw) false false)
        (`SceneComponent.K2_AddLocalRotation` (`self.Middle`) (`KismetMathLibrary.MakeRotator` 0.0 0.0 _returnvalue) false false)
        (goto _label)))))

(event `self.ReceiveTick`
  (params (DeltaSeconds :type "Float (single-precision)"))
  ;[1 1 1] Sphere Collision 중 어떤 것이라도 Target에 닿으면 불빛 켜짐
  (for (_array_element _array_index) (`self.TargetArr`)
    (for _array_element_2 (`self.CollisionArr`)
      (if (`PrimitiveComponent.IsOverlappingComponent` _array_element_2 _array_element)
        (bind _output (`|GetArrayItem` (`self.LightArr`) _array_index))
        (`SceneComponent.SetVisibility` _output true false)
        (break)
        (else
          (`SceneComponent.SetVisibility` _output false false))))))

(fn `UserConstructionScript`
  (`|ExecutionSequence`
    (:`then_0`
      (`KismetArrayLibrary.Array_Set` (`self.CollisionArr`) 0 (`self.Sphere1`))
      (`KismetArrayLibrary.Array_Set` (`self.CollisionArr`) 1 (`self.Sphere2`))
      (`KismetArrayLibrary.Array_Set` (`self.CollisionArr`) 2 (`self.Sphere3`))
      (`KismetArrayLibrary.Array_Set` (`self.CollisionArr`) 3 (`self.Sphere4`))
      (`KismetArrayLibrary.Array_Set` (`self.CollisionArr`) 4 (`self.DiffSphere`)))
    (:`then_1`
      (`KismetArrayLibrary.Array_Set` (`self.TargetArr`) 0 (`self.Target1`))
      (`KismetArrayLibrary.Array_Set` (`self.TargetArr`) 1 (`self.Target2`))
      (`KismetArrayLibrary.Array_Set` (`self.TargetArr`) 2 (`self.Target3`))
      (`KismetArrayLibrary.Array_Set` (`self.TargetArr`) 3 (`self.Target4`))
      (`KismetArrayLibrary.Array_Set` (`self.TargetArr`) 4 (`self.DiffTarget`)))
    (:`then_2`
      (`KismetArrayLibrary.Array_Set` (`self.LightArr`) 0 (`self.Light1`))
      (`KismetArrayLibrary.Array_Set` (`self.LightArr`) 1 (`self.Light2`))
      (`KismetArrayLibrary.Array_Set` (`self.LightArr`) 2 (`self.Light3`))
      (`KismetArrayLibrary.Array_Set` (`self.LightArr`) 3 (`self.Light4`))
      (`KismetArrayLibrary.Array_Set` (`self.LightArr`) 4 (`self.LightDiffT`)))))