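; BP_FirstInsideBox is a drag-operated puzzle box that moves through gated stages toward a collectible key.
; BlockMoving hands input from the Mover to the box until left mouse release.
; Mouse X slides the buttons and hexagon; Mouse Y rotates the CDs and moves the side drawers.
; Boolean flags chain the steps, timelines animate opening, and BP_ItemKey advances, gaining collision once the drawer finishes.
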(event `self.ReceiveBeginPlay`
  (bind _outactors (`GameplayStatics.GetAllActorsOfClass` "/Game/BoxesLike/BluePrints/RealBoxYuchin/BP_ItemKey.BP_ItemKey_C"))
  (set `self.KeyVar` (`|GetArrayItem` _outactors))
  (`PrimitiveComponent.SetCollisionEnabled` (`/Game/BoxesLike/BluePrints/RealBoxYuchin/BP_ItemKey.Key` (`self.KeyVar`)) "NoCollision"))

(event `/Game/BoxesLike/BPInterface/BlockMoving.Block Moving`
  (params (Mover :type "Pawn Object Reference") (ClickPoint :type "Vector Structure") (LookingComponentPoint :type "PrimitiveComponent Object Reference"))
  (bind _returnvalue (`GameplayStatics.GetPlayerController` 0))
  ;[1 1 1] 아이템 상세 확인 시작/종료 부분. 상세 확인을 시작하면 플레이어 캐릭터에 있던 컨트롤을 생성된 이 액터로 옮긴다.
  (if (or (== LookingComponentPoint (`self.GreenButton`)) (== LookingComponentPoint (`self.LeftCD`)) (== LookingComponentPoint (`self.RightCD`)) (== LookingComponentPoint (`self.Hexagon`)) (== LookingComponentPoint (`self.SideButton`)) (== LookingComponentPoint (`self.SideDowndrawer`)))
    (set `self.Looking Component Point` LookingComponentPoint)
    (`self.DisableInput` Mover _returnvalue)
    (`self.EnableInput` _returnvalue)))

(event `Key|LeftMouseButton`
  (params (Key :type "Key Structure"))
  (bind _returnvalue (`GameplayStatics.GetPlayerController` 0))
  ;[1 1 1] 아이템 상세 확인 시작/종료 부분. 상세 확인을 시작하면 플레이어 캐릭터에 있던 컨트롤을 생성된 이 액터로 옮긴다.
  (:`Released`
    (`self.DisableInput` _returnvalue)
    (`self.EnableInput` (stale `/Game/BoxesLike/BPInterface/BlockMoving.Block Moving` Mover) _returnvalue)))

(event `InputAxisKey|MouseX`
  (params (AxisValue :type "Float (single-precision)"))
  (bind (_relativelocation_x _relativelocation_y) (`KismetMathLibrary.BreakVector` (`SceneComponent.RelativeLocation` (`self.Hexagon`))))
  (bind (_relativelocation_x_2 _relativelocation_y_2) (`KismetMathLibrary.BreakVector` (`SceneComponent.RelativeLocation` (`self.GreenButton`))))
  (bind (_relativelocation_x_3 _relativelocation_y_3 _relativelocation_z) (`KismetMathLibrary.BreakVector` (`SceneComponent.RelativeLocation` (`self.Looking Component Point`))))
  (bind (_relativelocation_x_4 _relativelocation_y_4) (`KismetMathLibrary.BreakVector` (`SceneComponent.RelativeLocation` (`self.SideButton`))))
  ;[1 1 1] 마우스를 드래그하면 초록 버튼, Hexagon, Side Button y축(->)이동
  (if (`PlayerController.IsInputKeyDown` (`GameplayStatics.GetPlayerController` 0) "LeftMouseButton")
    (set `self.AxisValueX` (* AxisValue 0.25))
    (if (== (`self.Looking Component Point`) (`self.SideButton`))
      (set `self.AxisValueX` (* (`self.AxisValueX`) -1.0)))
    (if (or (and (<= _relativelocation_y_3 7.0) (>= _relativelocation_y_3 4.5) (`self.isButtonAct`) (== (`self.Looking Component Point`) (`self.GreenButton`))) (and (<= _relativelocation_y_3 1.5) (>= _relativelocation_y_3 -1.18) (`self.isHexagonAct`) (== (`self.Looking Component Point`) (`self.Hexagon`))) (and (<= _relativelocation_y_3 -3.5) (>= _relativelocation_y_3 -5.1) (`self.isSideBtAct`) (== (`self.Looking Component Point`) (`self.SideButton`))))
      (`SceneComponent.K2_SetRelativeLocation` (`self.Looking Component Point`) (`KismetMathLibrary.MakeVector` _relativelocation_x_3 (+ _relativelocation_y_3 (`self.AxisValueX`)) _relativelocation_z) false false)
      (if (and (>= _relativelocation_y_2 6.8) (`self.isButtonAct`))
        (`KismetSystemLibrary.Delay` 0.2)
        (`GameplayStatics.PlaySound2D` "/Game/BoxesLike/Sound/SE/Yuchin/FirstB_FrontDrawer_Cue.FirstB_FrontDrawer_Cue" 1.0 1.0 0.0 null null)
        (bind (_direction _btafteropen) (`Timeline|Timeline`)
          (:`Update`
            (`SceneComponent.K2_SetRelativeRotation` (`self.Open`) (`KismetMathLibrary.MakeRotator` 0.0 _btafteropen) false false))
          (:`Finished`
            (set `self.isButtonAct` false)
            (set `self.isWheelAct` true)))
        (elif (and (>= _relativelocation_y 1.45) (`self.isHexagonAct`))
          (set `self.canSQ` true)
          (`KismetSystemLibrary.Delay` 0.2)
          (`GameplayStatics.PlaySound2D` "/Game/BoxesLike/Sound/SE/Yuchin/FirstB_InsideBoxForward_Cue.FirstB_InsideBoxForward_Cue" 1.0 1.0 0.0 null null)
          (bind (_direction_2 _hexaafterboxmove) (`Timeline|Timeline_0`)
            (:`Update`
              (`SceneComponent.K2_SetRelativeLocation` (`self.MainBox`) (`KismetMathLibrary.MakeVector` _hexaafterboxmove) false false)
              (set `self.canSQ` false)
              (set `self.isHexagonAct` false))
            (:`Finished`
              (if (`/Game/BoxesLike/BluePrints/RealBoxYuchin/BP_ItemKey.isItemAct` (`self.KeyVar`))
                (`/Game/BoxesLike/BluePrints/RealBoxYuchin/BP_ItemKey.ItemGoForward` (`self.KeyVar`))
                (set `self.isSideBtAct` true))))
          (elif (and (>= _relativelocation_y_4 -3.6) (`self.isSideBtAct`))
            (set `self.isSideBtAct` false)
            (set `self.isSideDownDwAct` true)
            (`KismetSystemLibrary.PrintString` "sdd ready")))))))

(event `InputAxisKey|MouseY`
  (params (AxisValue :type "Float (single-precision)"))
  (bind _sidedowndrawer (`self.SideDowndrawer`))
  (bind (_relativelocation_x _relativelocation_y _relativelocation_z) (`KismetMathLibrary.BreakVector` (`SceneComponent.RelativeLocation` (`self.Looking Component Point`))))
  (bind _relativerotation_roll (`KismetMathLibrary.BreakRotator` (`SceneComponent.RelativeRotation` (`self.Looking Component Point`))))
  (bind (_relativerotation_roll_2 _relativerotation_pitch _relativerotation_yaw) (`KismetMathLibrary.BreakRotator` (`SceneComponent.RelativeRotation` (`self.Looking Component Point`))))
  (bind _relativerotation_roll_3 (`KismetMathLibrary.BreakRotator` (`SceneComponent.RelativeRotation` (`self.LeftCD`))))
  (bind (_relativelocation_x_2 _relativelocation_y_2 _relativelocation_z_2) (`KismetMathLibrary.BreakVector` (`SceneComponent.RelativeLocation` _sidedowndrawer)))
  (bind _relativerotation_roll_4 (`KismetMathLibrary.BreakRotator` (`SceneComponent.RelativeRotation` (`self.RightCD`))))
  (bind (_relativelocation_x_3 _relativelocation_y_3 _relativelocation_z_3) (`KismetMathLibrary.BreakVector` (`SceneComponent.RelativeLocation` (`self.SideDowndrawer`))))
  (bind (_relativerotation_roll_5 _relativerotation_pitch_2 _relativerotation_yaw_2) (`KismetMathLibrary.BreakRotator` (`SceneComponent.RelativeRotation` (`self.SideUpdrawer`))))
  ;[1 1 1] CD 2개 회전
  (if (`PlayerController.IsInputKeyDown` (`GameplayStatics.GetPlayerController` 0) "LeftMouseButton")
    (set `self.AxisValueY` (* AxisValue (`self.dir`)))
    (if (and (or (>= _relativerotation_roll 0.5) (<= _relativerotation_roll -0.5)) (`self.isWheelAct`) (or (== (`self.Looking Component Point`) (`self.LeftCD`)) (== (`self.Looking Component Point`) (`self.RightCD`))))
      (`GameplayStatics.PlaySound2D` "/Game/BoxesLike/Sound/SE/Yuchin/FirstB_CD_Cue.FirstB_CD_Cue" 1.0 1.0 0.0 null null)
      (`SceneComponent.K2_SetRelativeRotation` (`self.Looking Component Point`) (`KismetMathLibrary.MakeRotator` (+ _relativerotation_roll_2 (`self.AxisValueY`)) _relativerotation_pitch _relativerotation_yaw) false false)
      (if (and (or (>= _relativerotation_roll_3 -0.5) (<= _relativerotation_roll_3 0.5)) (or (>= _relativerotation_roll_4 -0.5) (<= _relativerotation_roll_4 0.5)))
        (set `self.isHexagonAct` true))
      (elif (and (== (`self.Looking Component Point`) _sidedowndrawer) (`self.isSideDownDwAct`) (>= _relativelocation_z_2 -4.0) (<= _relativelocation_z_2 0.6))
        (`SceneComponent.K2_SetRelativeLocation` (`self.Looking Component Point`) (`KismetMathLibrary.MakeVector` _relativelocation_x _relativelocation_y (+ _relativelocation_z (* (`self.AxisValueY`) -0.25))) false false)
        (`SceneComponent.K2_SetRelativeRotation` (`self.SideUpdrawer`) (`KismetMathLibrary.MakeRotator` _relativerotation_roll_5 (+ (* (`self.AxisValueY`) -5.0) _relativerotation_pitch_2) _relativerotation_yaw_2) false false)
        (if (>= _relativelocation_z_3 0.5)
          (`PrimitiveComponent.SetCollisionEnabled` (`/Game/BoxesLike/BluePrints/RealBoxYuchin/BP_ItemKey.Key` (`self.KeyVar`)) "QueryAndPhysics")
          (set `self.isSideDownDwAct` false))))))

(fn `UserConstructionScript`)