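; BP_ItemCompass is a compass pickup actor built from a body mesh and twelve light components.
; It starts hidden with collision disabled, and the CanAcquireCompass event makes it visible and collidable.
; GetItem returns the item's ID, name, texture and static mesh, and triggers DestroyItem.
; DestroyItem waits briefly before destroying the actor, leaving time for the return value and a possible pickup animation.
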(event `self.ReceiveBeginPlay`
  (`SceneComponent.SetVisibility` (`self.Body`) false false)
  (`SceneComponent.SetVisibility` (`self.Light5`) false false)
  (`SceneComponent.SetVisibility` (`self.Light4`) false false)
  (`SceneComponent.SetVisibility` (`self.Light3`) false false)
  (`SceneComponent.SetVisibility` (`self.Light2`) false false)
  (`SceneComponent.SetVisibility` (`self.Light6`) false false)
  (`SceneComponent.SetVisibility` (`self.Light12`) false false)
  (`SceneComponent.SetVisibility` (`self.Light1`) false false)
  (`SceneComponent.SetVisibility` (`self.Light7`) false false)
  (`SceneComponent.SetVisibility` (`self.Light11`) false false)
  (`SceneComponent.SetVisibility` (`self.Light8`) false false)
  (`SceneComponent.SetVisibility` (`self.Light9`) false false)
  (`SceneComponent.SetVisibility` (`self.Light10`) false false)
  (`PrimitiveComponent.SetCollisionEnabled` (`self.Body`) "NoCollision")
  (`PrimitiveComponent.SetCollisionEnabled` (`self.Light5`) "NoCollision")
  (`PrimitiveComponent.SetCollisionEnabled` (`self.Light4`) "NoCollision")
  (`PrimitiveComponent.SetCollisionEnabled` (`self.Light3`) "NoCollision")
  (`PrimitiveComponent.SetCollisionEnabled` (`self.Light2`) "NoCollision")
  (`PrimitiveComponent.SetCollisionEnabled` (`self.Light6`) "NoCollision")
  (`PrimitiveComponent.SetCollisionEnabled` (`self.Light12`) "NoCollision")
  (`PrimitiveComponent.SetCollisionEnabled` (`self.Light1`) "NoCollision")
  (`PrimitiveComponent.SetCollisionEnabled` (`self.Light7`) "NoCollision")
  (`PrimitiveComponent.SetCollisionEnabled` (`self.Light11`) "NoCollision")
  (`PrimitiveComponent.SetCollisionEnabled` (`self.Light8`) "NoCollision")
  (`PrimitiveComponent.SetCollisionEnabled` (`self.Light9`) "NoCollision")
  (`PrimitiveComponent.SetCollisionEnabled` (`self.Light10`) "NoCollision"))

(event `CanAcquireCompass`
  (`SceneComponent.SetVisibility` (`self.Body`) true false)
  (`SceneComponent.SetVisibility` (`self.Light5`) true false)
  (`SceneComponent.SetVisibility` (`self.Light4`) true false)
  (`SceneComponent.SetVisibility` (`self.Light3`) true false)
  (`SceneComponent.SetVisibility` (`self.Light2`) true false)
  (`SceneComponent.SetVisibility` (`self.Light6`) true false)
  (`SceneComponent.SetVisibility` (`self.Light12`) true false)
  (`SceneComponent.SetVisibility` (`self.Light1`) true false)
  (`SceneComponent.SetVisibility` (`self.Light7`) true false)
  (`SceneComponent.SetVisibility` (`self.Light11`) true false)
  (`SceneComponent.SetVisibility` (`self.Light8`) true false)
  (`SceneComponent.SetVisibility` (`self.Light9`) true false)
  (`SceneComponent.SetVisibility` (`self.Light10`) true false)
  (`PrimitiveComponent.SetCollisionEnabled` (`self.Body`) "QueryAndPhysics")
  (`PrimitiveComponent.SetCollisionEnabled` (`self.Light5`) "QueryAndPhysics")
  (`PrimitiveComponent.SetCollisionEnabled` (`self.Light4`) "QueryAndPhysics")
  (`PrimitiveComponent.SetCollisionEnabled` (`self.Light3`) "QueryAndPhysics")
  (`PrimitiveComponent.SetCollisionEnabled` (`self.Light2`) "QueryAndPhysics")
  (`PrimitiveComponent.SetCollisionEnabled` (`self.Light6`) "QueryAndPhysics")
  (`PrimitiveComponent.SetCollisionEnabled` (`self.Light12`) "QueryAndPhysics")
  (`PrimitiveComponent.SetCollisionEnabled` (`self.Light1`) "QueryAndPhysics")
  (`PrimitiveComponent.SetCollisionEnabled` (`self.Light7`) "QueryAndPhysics")
  (`PrimitiveComponent.SetCollisionEnabled` (`self.Light11`) "QueryAndPhysics")
  (`PrimitiveComponent.SetCollisionEnabled` (`self.Light8`) "QueryAndPhysics")
  (`PrimitiveComponent.SetCollisionEnabled` (`self.Light9`) "QueryAndPhysics")
  (`PrimitiveComponent.SetCollisionEnabled` (`self.Light10`) "QueryAndPhysics"))

(event `DestroyItem`
  ;[1 1 1] 아이템 획득시 딜레이를 줘서 액터 삭제 전 리턴값을 줄 시간을 얻음.
  ; 액터 삭제 전 획득 애니메이션 삽입 가능
  (`KismetSystemLibrary.Delay` 0.2)
  (`KismetSystemLibrary.PrintString` "Compass Acquired")
  (`self.K2_DestroyActor`))

(fn `GetItem`
  (returns (ItemID :type Integer) (ItemName :type String) (ItemTexture :type "Texture2D Object Reference") (ItemStaticMesh :type "StaticMesh Object Reference"))
  (`self.DestroyItem`)
  (return (`self.ItemId`) (`self.ItemName`) (`self.ItemTexture`) (`self.ItemStaticMesh`)))

(fn `UserConstructionScript`)