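; BP_Door is a puzzle door that opens via the DoorFall timeline when four pieces overlap their answer volumes.
; BlockMoving shifts input from the Mover to this actor, so mouse drags slide pieces within clamped ranges until release.
; The button rotates ShapePieces 90 degrees for limited presses, with turn parity remapping mouse axes.
; Tick detaches or reparents pieces by AnswerCollision overlap and triggers the answer check.
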(event `/Game/BoxesLike/BPInterface/BlockMoving.Block Moving`
  (params (Mover :type "Pawn Object Reference") (ClickPoint :type "Vector Structure") (LookingComponentPoint :type "PrimitiveComponent Object Reference"))
  (bind _returnvalue (`GameplayStatics.GetPlayerController` 0))
  ;[1 1 1] 플레이어 캐릭터에 있던 컨트롤을 생성된 이 액터로 옮긴다.
  (if (or (== LookingComponentPoint (`self.piece0`)) (== LookingComponentPoint (`self.piece1`)) (== LookingComponentPoint (`self.piece2`)) (== LookingComponentPoint (`self.piece3`)))
    (set `self.LookingComponentPoint` LookingComponentPoint)
    (`self.DisableInput` Mover _returnvalue)
    (`self.EnableInput` _returnvalue)))

(event `Key|LeftMouseButton`
  (params (Key :type "Key Structure"))
  (bind _returnvalue (`GameplayStatics.GetPlayerController` 0))
  ;[1 1 1] 플레이어 캐릭터에 있던 컨트롤을 생성된 이 액터로 옮긴다.
  (:`Released`
    (`self.DisableInput` _returnvalue)
    (`self.EnableInput` (stale `/Game/BoxesLike/BPInterface/BlockMoving.Block Moving` Mover) _returnvalue)))

(event `self.ReceiveBeginPlay`
  (set `PlayerController.bEnableClickEvents` true (`GameplayStatics.GetPlayerController` 0))
  (`PrimitiveComponent.SetCollisionEnabled` (`self.Arch`) "NoCollision")
  (`PrimitiveComponent.SetCollisionEnabled` (`self.Door`) "NoCollision") ; 충돌 삭제 안 하면 조각들 클릭이 안 먹음
  (`self.FindAnswer`))

(event `self.Button.OnClicked`
  (params (TouchedComponent :type "PrimitiveComponent Object Reference") (ButtonPressed :type "Key Structure"))
  ;[1 1 1] 가운데 버튼 누르면 90도 회전
  (bind _output_get (set `self.startRotation` (`SceneComponent.RelativeRotation` (`self.ShapePieces`))))
  (set `self.endRotation` (`KismetMathLibrary.ComposeRotators` _output_get (struct :`Pitch` 90.0)))
  (if (<= (`self.cnt`) 10)
    (bind (_direction _rotate) (`Timeline|Rotate90` :!via `PlayFromStart`)
      (:`Update`
        (`SceneComponent.K2_SetRelativeRotation` (`self.ShapePieces`) (`KismetMathLibrary.RLerp` (`self.startRotation`) (`self.endRotation`) (* _rotate -1.0) true) false false))
      (:`Finished`
        (set `self.cnt` (+ (`self.cnt`) 1))
        (set `self.isRotate` true)
        (if (== (mod (`self.cnt`) 2) 1)
          (set `self.p02` true)
          (set `self.p13` false)
          (else
            (set `self.p13` true)
            (set `self.p02` false)))))))

(event `InputAxisKey|MouseY`
  (params (AxisValue :type "Float (single-precision)"))
  (bind _lookingcomponentpoint (`self.LookingComponentPoint`))
  (bind _lookingcomponentpoint_2 (`self.LookingComponentPoint`))
  (bind _axisy_z_getlocplus (`self.AxisY_Z getLocPlus`))
  (bind _axisy_z_getlocplus_2 (`self.AxisY_Z getLocPlus`))
  (bind _lookingcomponentpoint_3 (`self.LookingComponentPoint`))
  (bind _lookingcomponentpoint_4 (`self.LookingComponentPoint`))
  (bind _lookingcomponentpoint_5 (`self.LookingComponentPoint`))
  (bind _lookingcomponentpoint_6 (`self.LookingComponentPoint`))
  (bind _axisy_x_getlocplus (`self.AxisY_X getLocPlus`))
  (bind _axisy_x_getlocplus_2 (`self.AxisY_X getLocPlus`))
  (bind (_relativelocation_x _relativelocation_y) (`KismetMathLibrary.BreakVector` (`SceneComponent.RelativeLocation` _lookingcomponentpoint)))
  (bind (_relativelocation_x_2 _relativelocation_y_2) (`KismetMathLibrary.BreakVector` (`SceneComponent.RelativeLocation` _lookingcomponentpoint)))
  (bind (_relativelocation_x_3 _relativelocation_y_3) (`KismetMathLibrary.BreakVector` (`SceneComponent.RelativeLocation` _lookingcomponentpoint_2)))
  (bind (_relativelocation_x_4 _relativelocation_y_4) (`KismetMathLibrary.BreakVector` (`SceneComponent.RelativeLocation` _lookingcomponentpoint_2)))
  (bind (_relativelocation_x_5 _relativelocation_y_5 _relativelocation_z) (`KismetMathLibrary.BreakVector` (`SceneComponent.RelativeLocation` (`self.LookingComponentPoint`))))
  (bind (_relativelocation_x_6 _relativelocation_y_6 _relativelocation_z_2) (`KismetMathLibrary.BreakVector` (`SceneComponent.RelativeLocation` _lookingcomponentpoint_3)))
  (bind _relativelocation_x_7 (`KismetMathLibrary.BreakVector` (`SceneComponent.RelativeLocation` (`self.LookingComponentPoint`))))
  (bind (_relativelocation_x_8 _relativelocation_y_7 _relativelocation_z_3) (`KismetMathLibrary.BreakVector` (`SceneComponent.RelativeLocation` _lookingcomponentpoint_4)))
  (bind (_relativelocation_x_9 _relativelocation_y_8 _relativelocation_z_4) (`KismetMathLibrary.BreakVector` (`SceneComponent.RelativeLocation` _lookingcomponentpoint_5)))
  (bind (_relativelocation_x_10 _relativelocation_y_9 _relativelocation_z_5) (`KismetMathLibrary.BreakVector` (`SceneComponent.RelativeLocation` _lookingcomponentpoint_5)))
  (bind (_relativelocation_x_11 _relativelocation_y_10 _relativelocation_z_6) (`KismetMathLibrary.BreakVector` (`SceneComponent.RelativeLocation` _lookingcomponentpoint_6)))
  (bind (_relativelocation_x_12 _relativelocation_y_11 _relativelocation_z_7) (`KismetMathLibrary.BreakVector` (`SceneComponent.RelativeLocation` _lookingcomponentpoint_6)))
  (bind _returnvalue (`KismetMathLibrary.Abs` _relativelocation_z))
  (bind _returnvalue_2 (`KismetMathLibrary.Abs` _relativelocation_x_7))
  (bind _returnvalue_3 (+ _relativelocation_x_8 (* (`self.AxisValueY`) -0.25)))
  (bind _returnvalue_4 (+ _relativelocation_z_2 (* (`self.AxisValueY`) 0.25)))
  ;[1 1 1] p1,p3 또는 p0,p2가 세로방향으로 움직일때 (이때 움직이는 방향은p1,p3은 x축이고 p0,p2는 z축임)
  (set `self.AxisValueY` AxisValue)
  (if (`PlayerController.IsInputKeyDown` (`GameplayStatics.GetPlayerController` 0) "LeftMouseButton")
    (if (or (== (`self.LookingComponentPoint`) (`self.piece1`)) (== (`self.LookingComponentPoint`) (`self.piece3`)))
      (if (not (and (`self.p13`) (<= _returnvalue_2 12.5) (>= _returnvalue_2 3.3)))
        (set `self.AxisY_X getLocPlus` _returnvalue_3)
        (`SceneComponent.K2_SetRelativeLocation` _lookingcomponentpoint_4 (`KismetMathLibrary.MakeVector` _returnvalue_3 _relativelocation_y_7 _relativelocation_z_3) false false)
        (if (and (> _axisy_x_getlocplus 0.0) (<= _axisy_x_getlocplus 3.8))
          (`SceneComponent.K2_SetRelativeLocation` _lookingcomponentpoint_5 (`KismetMathLibrary.MakeVector` 3.8 _relativelocation_y_8 _relativelocation_z_4) false false)
          (elif (>= (`self.AxisY_X getLocPlus`) 12.0)
            (`SceneComponent.K2_SetRelativeLocation` _lookingcomponentpoint_5 (`KismetMathLibrary.MakeVector` 12.0 _relativelocation_y_9 _relativelocation_z_5) false false)
            (elif (and (< _axisy_x_getlocplus_2 0.0) (>= _axisy_x_getlocplus_2 -3.8))
              (`SceneComponent.K2_SetRelativeLocation` _lookingcomponentpoint_6 (`KismetMathLibrary.MakeVector` -3.8 _relativelocation_y_10 _relativelocation_z_6) false false)
              (elif (<= (`self.AxisY_X getLocPlus`) -12.0)
                (`SceneComponent.K2_SetRelativeLocation` _lookingcomponentpoint_6 (`KismetMathLibrary.MakeVector` -12.0 _relativelocation_y_11 _relativelocation_z_7) false false))))))
      (elif (or (== (`self.LookingComponentPoint`) (`self.piece0`)) (== (`self.LookingComponentPoint`) (`self.piece2`)))
        (if (not (and (`self.p02`) (<= _returnvalue 12.5) (>= _returnvalue 3.3)))
          (set `self.AxisY_Z getLocPlus` _returnvalue_4)
          (`SceneComponent.K2_SetRelativeLocation` _lookingcomponentpoint_3 (`KismetMathLibrary.MakeVector` _relativelocation_x_6 _relativelocation_y_6 _returnvalue_4) false false)
          (if (and (> _axisy_z_getlocplus 0.0) (<= _axisy_z_getlocplus 3.8))
            (`SceneComponent.K2_SetRelativeLocation` _lookingcomponentpoint (`KismetMathLibrary.MakeVector` _relativelocation_x _relativelocation_y 3.8) false false)
            (elif (>= (`self.AxisY_Z getLocPlus`) 12.0)
              (`SceneComponent.K2_SetRelativeLocation` _lookingcomponentpoint (`KismetMathLibrary.MakeVector` _relativelocation_x_2 _relativelocation_y_2 12.0) false false)
              (elif (and (< _axisy_z_getlocplus_2 0.0) (>= _axisy_z_getlocplus_2 -3.8))
                (`SceneComponent.K2_SetRelativeLocation` _lookingcomponentpoint_2 (`KismetMathLibrary.MakeVector` _relativelocation_x_3 _relativelocation_y_3 -3.8) false false)
                (elif (<= (`self.AxisY_Z getLocPlus`) -12.0)
                  (`SceneComponent.K2_SetRelativeLocation` _lookingcomponentpoint_2 (`KismetMathLibrary.MakeVector` _relativelocation_x_4 _relativelocation_y_4 -12.0) false false))))))))))

(event `InputAxisKey|MouseX`
  (params (AxisValue :type "Float (single-precision)"))
  (bind _lookingcomponentpoint (`self.LookingComponentPoint`))
  (bind _lookingcomponentpoint_2 (`self.LookingComponentPoint`))
  (bind _axisx_x_getlocplus (`self.AxisX_X getLocPlus`))
  (bind _axisx_x_getlocplus_2 (`self.AxisX_X getLocPlus`))
  (bind _axisx_z_getlocplus (`self.AxisX_Z getLocPlus`))
  (bind _axisx_z_getlocplus_2 (`self.AxisX_Z getLocPlus`))
  (bind _lookingcomponentpoint_3 (`self.LookingComponentPoint`))
  (bind _lookingcomponentpoint_4 (`self.LookingComponentPoint`))
  (bind _lookingcomponentpoint_5 (`self.LookingComponentPoint`))
  (bind _lookingcomponentpoint_6 (`self.LookingComponentPoint`))
  (bind _relativelocation_x (`KismetMathLibrary.BreakVector` (`SceneComponent.RelativeLocation` (`self.LookingComponentPoint`))))
  (bind (_relativelocation_x_2 _relativelocation_y _relativelocation_z) (`KismetMathLibrary.BreakVector` (`SceneComponent.RelativeLocation` _lookingcomponentpoint)))
  (bind (_relativelocation_x_3 _relativelocation_y_2 _relativelocation_z_2) (`KismetMathLibrary.BreakVector` (`SceneComponent.RelativeLocation` _lookingcomponentpoint)))
  (bind (_relativelocation_x_4 _relativelocation_y_3 _relativelocation_z_3) (`KismetMathLibrary.BreakVector` (`SceneComponent.RelativeLocation` _lookingcomponentpoint_2)))
  (bind (_relativelocation_x_5 _relativelocation_y_4 _relativelocation_z_4) (`KismetMathLibrary.BreakVector` (`SceneComponent.RelativeLocation` _lookingcomponentpoint_2)))
  (bind (_relativelocation_x_6 _relativelocation_y_5 _relativelocation_z_5) (`KismetMathLibrary.BreakVector` (`SceneComponent.RelativeLocation` _lookingcomponentpoint_3)))
  (bind (_relativelocation_x_7 _relativelocation_y_6 _relativelocation_z_6) (`KismetMathLibrary.BreakVector` (`SceneComponent.RelativeLocation` (`self.LookingComponentPoint`))))
  (bind (_relativelocation_x_8 _relativelocation_y_7 _relativelocation_z_7) (`KismetMathLibrary.BreakVector` (`SceneComponent.RelativeLocation` _lookingcomponentpoint_4)))
  (bind (_relativelocation_x_9 _relativelocation_y_8) (`KismetMathLibrary.BreakVector` (`SceneComponent.RelativeLocation` _lookingcomponentpoint_5)))
  (bind (_relativelocation_x_10 _relativelocation_y_9) (`KismetMathLibrary.BreakVector` (`SceneComponent.RelativeLocation` _lookingcomponentpoint_5)))
  (bind (_relativelocation_x_11 _relativelocation_y_10) (`KismetMathLibrary.BreakVector` (`SceneComponent.RelativeLocation` _lookingcomponentpoint_6)))
  (bind (_relativelocation_x_12 _relativelocation_y_11) (`KismetMathLibrary.BreakVector` (`SceneComponent.RelativeLocation` _lookingcomponentpoint_6)))
  (bind _returnvalue (`KismetMathLibrary.Abs` _relativelocation_x))
  (bind _returnvalue_2 (`KismetMathLibrary.Abs` _relativelocation_z_6))
  (bind _returnvalue_3 (+ _relativelocation_x_6 (* (`self.AxisValueX`) 0.25)))
  (bind _returnvalue_4 (+ _relativelocation_z_7 (* (`self.AxisValueX`) -0.25)))
  ;[1 1 1] p1,p3 또는 p0,p2가 가로방향으로 움직일때 (이때 움직이는 방향은p1,p3은 x축이고 p0,p2는 z축임)
  (set `self.AxisValueX` AxisValue)
  (if (`PlayerController.IsInputKeyDown` (`GameplayStatics.GetPlayerController` 0) "LeftMouseButton")
    (if (or (== (`self.LookingComponentPoint`) (`self.piece1`)) (== (`self.LookingComponentPoint`) (`self.piece3`)))
      (if (and (`self.p13`) (<= _returnvalue 12.5) (>= _returnvalue 3.3))
        (set `self.AxisX_X getLocPlus` _returnvalue_3)
        (`SceneComponent.K2_SetRelativeLocation` _lookingcomponentpoint_3 (`KismetMathLibrary.MakeVector` _returnvalue_3 _relativelocation_y_5 _relativelocation_z_5) false false)
        (if (and (> _axisx_x_getlocplus 0.0) (<= _axisx_x_getlocplus 3.8))
          (`SceneComponent.K2_SetRelativeLocation` _lookingcomponentpoint (`KismetMathLibrary.MakeVector` 3.8 _relativelocation_y _relativelocation_z) false false)
          (elif (>= (`self.AxisX_X getLocPlus`) 12.0)
            (`SceneComponent.K2_SetRelativeLocation` _lookingcomponentpoint (`KismetMathLibrary.MakeVector` 12.0 _relativelocation_y_2 _relativelocation_z_2) false false)
            (elif (and (< _axisx_x_getlocplus_2 0.0) (>= _axisx_x_getlocplus_2 -3.8))
              (`SceneComponent.K2_SetRelativeLocation` _lookingcomponentpoint_2 (`KismetMathLibrary.MakeVector` -3.8 _relativelocation_y_3 _relativelocation_z_3) false false)
              (elif (<= (`self.AxisX_X getLocPlus`) -12.0)
                (`SceneComponent.K2_SetRelativeLocation` _lookingcomponentpoint_2 (`KismetMathLibrary.MakeVector` -12.0 _relativelocation_y_4 _relativelocation_z_4) false false))))))
      (elif (or (== (`self.LookingComponentPoint`) (`self.piece0`)) (== (`self.LookingComponentPoint`) (`self.piece2`)))
        (if (and (`self.p02`) (<= _returnvalue_2 12.5) (>= _returnvalue_2 3.3))
          (set `self.AxisX_Z getLocPlus` _returnvalue_4)
          (`SceneComponent.K2_SetRelativeLocation` _lookingcomponentpoint_4 (`KismetMathLibrary.MakeVector` _relativelocation_x_8 _relativelocation_y_7 _returnvalue_4) false false)
          (if (and (> _axisx_z_getlocplus 0.0) (<= _axisx_z_getlocplus 3.8))
            (`SceneComponent.K2_SetRelativeLocation` _lookingcomponentpoint_5 (`KismetMathLibrary.MakeVector` _relativelocation_x_9 _relativelocation_y_8 3.8) false false)
            (elif (>= (`self.AxisX_Z getLocPlus`) 12.0)
              (`SceneComponent.K2_SetRelativeLocation` _lookingcomponentpoint_5 (`KismetMathLibrary.MakeVector` _relativelocation_x_10 _relativelocation_y_9 12.0) false false)
              (elif (and (< _axisx_z_getlocplus_2 0.0) (>= _axisx_z_getlocplus_2 -3.8))
                (`SceneComponent.K2_SetRelativeLocation` _lookingcomponentpoint_6 (`KismetMathLibrary.MakeVector` _relativelocation_x_11 _relativelocation_y_10 -3.8) false false)
                (elif (<= (`self.AxisX_Z getLocPlus`) -12.0)
                  (`SceneComponent.K2_SetRelativeLocation` _lookingcomponentpoint_6 (`KismetMathLibrary.MakeVector` _relativelocation_x_12 _relativelocation_y_11 -12.0) false false))))))))))

(event `FindAnswer`)

(event `self.ReceiveTick`
  (params (DeltaSeconds :type "Float (single-precision)"))
  (if (`PrimitiveComponent.IsOverlappingComponent` (`self.AnswerCollision`) (`self.p0_Collision`))
    (set `self.p0` true)
    (else
      (set `self.p0` false)))
  (if (`self.p0`)
    (`SceneComponent.K2_DetachFromComponent` (`self.piece0`) "KeepRelative" "KeepRelative" "KeepRelative" true)
    (`self.CheckAnswer`)
    (else
      (`SceneComponent.K2_AttachToComponent` (`self.piece0`) (`self.ShapePieces`) "None" "KeepRelative" "KeepRelative" "KeepRelative" true)))
  (if (`PrimitiveComponent.IsOverlappingComponent` (`self.AnswerCollision`) (`self.p1_Collision`))
    (set `self.p1` true)
    (else
      (set `self.p1` false)))
  (if (`self.p1`)
    (`SceneComponent.K2_AttachToComponent` (`self.piece1`) (`self.Answer`) "None" "KeepRelative" "KeepRelative" "KeepRelative" true)
    (`self.CheckAnswer`)
    (else
      (`SceneComponent.K2_AttachToComponent` (`self.piece1`) (`self.ShapePieces`) "None" "KeepRelative" "KeepRelative" "KeepRelative" true)))
  (if (`PrimitiveComponent.IsOverlappingComponent` (`self.AnswerCollision`) (`self.p2_Collision`))
    (set `self.p2` true)
    (else
      (set `self.p2` false)))
  (if (`self.p2`)
    (`SceneComponent.K2_AttachToComponent` (`self.piece2`) (`self.Answer`) "None" "KeepRelative" "KeepRelative" "KeepRelative" true)
    (`self.CheckAnswer`)
    (else
      (`SceneComponent.K2_AttachToComponent` (`self.piece2`) (`self.ShapePieces`) "None" "KeepRelative" "KeepRelative" "KeepRelative" true)))
  (if (`PrimitiveComponent.IsOverlappingComponent` (`self.AnswerCollision`) (`self.p3_Collision`))
    (set `self.p3` true)
    (else
      (set `self.p3` false)))
  (if (`self.p3`)
    (`SceneComponent.K2_AttachToComponent` (`self.piece3`) (`self.Answer`) "None" "KeepRelative" "KeepRelative" "KeepRelative" true)
    (`self.CheckAnswer`)
    (else
      (`SceneComponent.K2_AttachToComponent` (`self.piece3`) (`self.ShapePieces`) "None" "KeepRelative" "KeepRelative" "KeepRelative" true))))

(event `CheckAnswer`
  (bind _door (`self.Door`))
  (bind (_relativelocation_x _relativelocation_y) (`KismetMathLibrary.BreakVector` (`SceneComponent.RelativeLocation` _door)))
  (if (and (`PrimitiveComponent.IsOverlappingComponent` (`self.p0_Collision`) (`self.p0_answer`)) (`PrimitiveComponent.IsOverlappingComponent` (`self.p1_Collision`) (`self.p1_answer`)) (`PrimitiveComponent.IsOverlappingComponent` (`self.p2_Collision`) (`self.p2_answer`)) (`PrimitiveComponent.IsOverlappingComponent` (`self.p3_Collision`) (`self.p3_answer`)))
    (`KismetSystemLibrary.PrintString` "Correct")
    (bind (_direction _fall) (`Timeline|DoorFall`)
      (:`Update`
        (`SceneComponent.K2_SetRelativeLocation` _door (`KismetMathLibrary.MakeVector` _relativelocation_x _relativelocation_y _fall) false false)))))

(fn `UserConstructionScript`)