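; BP_ItemKey is a pickup key item that hands its item data to the caller and removes itself.
; GetItem triggers DestoryItem and returns the ID, name, texture and static mesh.
; DestoryItem waits briefly before printing an acquired message and destroying the actor, so the return completes first and an acquisition animation could fit in.
; ItemGoForward shifts the key mesh along world X and clears IsItemAct.
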(event `ItemGoForward`
  (bind _key (`self.Key`))
  (bind (_returnvalue_x _returnvalue_y _returnvalue_z) (`KismetMathLibrary.BreakVector` (`SceneComponent.K2_GetComponentLocation` _key)))
  (`SceneComponent.K2_SetWorldLocation` _key (`KismetMathLibrary.MakeVector` (+ _returnvalue_x -37.0) _returnvalue_y _returnvalue_z) false false)
  (set `self.isItemAct` false))

(event `DestoryItem`
  ;[1 1 1] 아이템 획득시 딜레이를 줘서 액터 삭제 전 리턴값을 줄 시간을 얻음.
  ; 액터 삭제 전 획득 애니메이션 삽입 가능
  (`KismetSystemLibrary.Delay` 0.2)
  (`KismetSystemLibrary.PrintString` "Key Acquired")
  (`self.K2_DestroyActor`))

(fn `GetItem`
  (returns (ItemID :type Integer) (ItemName :type String) (ItemTexture :type "Texture2D Object Reference") (ItemStaticMesh :type "StaticMesh Object Reference"))
  (`self.DestoryItem`)
  (return (`self.ItemId`) (`self.ItemName`) (`self.ItemTexture`) (`self.ItemStaticMesh`)))

(fn `UserConstructionScript`)