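; BP_NameWidget1 is an actor whose Widget component turns to face the player's camera, apparently as a floating name label.
; BeginPlay caches the first BP_ChallengersCharacter found in the world.
; Each Tick billboards the widget toward that character's FollowCamera using MakeRotFromZX, with world up as Z so it stays upright.
; If the character or camera is invalid, Tick repeats the lookup.
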(event `self.ReceiveBeginPlay`
  (bind _returnvalue (`GameplayStatics.GetActorOfClass` "/Game/Yuchin/Blueprints/BP_ChallengersCharacter.BP_ChallengersCharacter_C" :!label _label))
  (set `self.PlayerREF` _returnvalue))

(event `self.ReceiveTick`
  (params (DeltaSeconds :type "Float (single-precision)"))
  (bind _widget (`self.Widget`))
  (bind _followcamera (`ChallengersCharacter.FollowCamera` (`self.PlayerREF`)))
  (`/Engine/EditorBlueprintResources/StandardMacros.IsValid` (`self.PlayerREF`)
    (:`Is Valid`
      (`/Engine/EditorBlueprintResources/StandardMacros.IsValid` _followcamera
        (:`Is Valid`
          (`SceneComponent.K2_SetWorldRotation` _widget (`KismetMathLibrary.MakeRotFromZX` (`KismetMathLibrary.GetUpVector` (struct)) (- (`SceneComponent.K2_GetComponentLocation` _followcamera) (`SceneComponent.K2_GetComponentLocation` _widget))) false false))
        (:`Is Not Valid`
          (goto _label))))
    (:`Is Not Valid`
      (goto _label))))

(fn `UserConstructionScript`)