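; BP_ChallengersCharacter is a character Blueprint whose only active logic limits how far the player camera can look up and down.
; On BeginPlay it sets a symmetric pitch clamp on player 0's camera manager.
; The construction script does nothing, as its nodes attaching sword, wand and gun components to matching mesh sockets are disconnected and never run.
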(event `self.ReceiveBeginPlay`
  (bind _returnvalue (`GameplayStatics.GetPlayerCameraManager` 0))
  (set `PlayerCameraManager.ViewPitchMin` -40.0 _returnvalue)
  (set `PlayerCameraManager.ViewPitchMax` 40.0 _returnvalue))

(fn `UserConstructionScript`)