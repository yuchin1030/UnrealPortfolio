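; Test trigger actor that loads saved enemy data onto a referenced enemy when a ChallengersCharacter overlaps its box.
; On overlap, it has OurGameInstance load the enemy list, then searches it for EnemyName to build EnemyREF's spec.
; The loop's current entry then supplies body, weapon, gear and AI data to LoadData, and its battle distance is printed.
; The construction script shows EnemyName on a text render.
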(event `self.ReceiveBeginPlay`)

(event `self.Box.OnComponentBeginOverlap`
  (params (OverlappedComponent :type "PrimitiveComponent Object Reference") (OtherActor :type "Actor Object Reference") (OtherComp :type "PrimitiveComponent Object Reference") (OtherBodyIndex :type Integer) (bFromSweep :type Boolean) (SweepResult :type "HitResult Structure (by ref)"))
  (bind _enemyref (`self.EnemyREF`))
  (cast `ChallengersCharacter` OtherActor)
  (bind _asour_game_instance (cast `OurGameInstance` (`GameplayStatics.GetGameInstance`)))
  (`OurGameInstance.LoadEnemyData` _asour_game_instance)
  (for _array_element (`OurGameInstance.loadedEnemyDataList` _asour_game_instance)
    (bind (_name _bisbosstype _totalcost _bodyrowname _weapon1rowname _weapon2rowname _gearrowname _aidata) (break `EnemySaveDataStruct` _array_element))
    (if (`KismetStringLibrary.EqualEqual_StrStr` (`self.enemyName`) _name)
      (set `BaseEnemy.enemySpec` (make `spec` _name _bisbosstype 0 0 0 0.0 0 0 _totalcost) _enemyref)
      (break)))
  (`BaseEnemy.LoadData` _enemyref _bodyrowname _weapon1rowname _weapon2rowname _gearrowname _aidata)
  (`KismetSystemLibrary.PrintString` (`KismetStringLibrary.Conv_DoubleToString` (`.battleDist` (break `AIStat` _aidata)))))

(fn `UserConstructionScript`
  (`TextRenderComponent.K2_SetText` (`self.TextRender`) (`KismetTextLibrary.Conv_StringToText` (`self.enemyName`))))