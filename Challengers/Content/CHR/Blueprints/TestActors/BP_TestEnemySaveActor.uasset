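; Test actor that saves a referenced enemy's configuration when a ChallengersCharacter overlaps its box.
; On overlap it passes the enemy's boss flag, total cost, body, weapon and gear row names, and AI data to SaveEnemyData on OurGameInstance, under the actor's EnemyName.
; The construction script shows EnemyName on a text render as a label.
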(event `self.ReceiveBeginPlay`)

(event `self.Box.OnComponentBeginOverlap`
  (params (OverlappedComponent :type "PrimitiveComponent Object Reference") (OtherActor :type "Actor Object Reference") (OtherComp :type "PrimitiveComponent Object Reference") (OtherBodyIndex :type Integer) (bFromSweep :type Boolean) (SweepResult :type "HitResult Structure (by ref)"))
  (bind _enemyref (`self.EnemyREF`))
  (bind (_enemyspec_name _enemyspec_bisbosstype _enemyspec_totalhp _enemyspec_totalattackpoint _enemyspec_totaldef _enemyspec_speed _enemyspec_weightlimit _enemyspec_currentweight _enemyspec_totalcost) (break `spec` (`BaseEnemy.enemySpec` _enemyref)))
  (cast `ChallengersCharacter` OtherActor)
  (bind _asour_game_instance (cast `OurGameInstance` (`GameplayStatics.GetGameInstance`)))
  (`OurGameInstance.SaveEnemyData` _asour_game_instance (`self.enemyName`) _enemyspec_bisbosstype _enemyspec_totalcost (`BaseEnemy.bodyRowName` _enemyref) (`BaseEnemy.weapon1RowName` _enemyref) (`BaseEnemy.weapon2RowName` _enemyref) (`BaseEnemy.gearRowName` _enemyref) (`BaseEnemy.AIData` _enemyref)))

(fn `UserConstructionScript`
  (`TextRenderComponent.K2_SetText` (`self.TextRender`) (`KismetTextLibrary.Conv_StringToText` (`self.enemyName`))))