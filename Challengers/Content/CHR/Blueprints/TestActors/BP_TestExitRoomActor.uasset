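; Test exit-room actor that sends players out of the multiplayer session and into SingleMap when a challenger character enters its sphere.
; A floating "<EXIT>" widget turns each tick toward the follow camera of the character found at BeginPlay.
; Overlap branches on authority: host loops over all player controllers, client uses the character's own.
; Both fade the camera, delay, destroy the session, flag loading on the game instance and open the map.
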(event `self.ReceiveBeginPlay`
  (bind _returnvalue (`GameplayStatics.GetActorOfClass` "/Game/Yuchin/Blueprints/BP_ChallengersCharacter.BP_ChallengersCharacter_C"))
  (set `self.PlayerREF` _returnvalue)
  (bind _asname_bill_board_widget (cast `NameBillBoardWidget` (`WidgetComponent.GetWidget` (`self.floatingNameComp`))))
  (`TextBlock.SetText` (`NameBillBoardWidget.name` _asname_bill_board_widget) "<EXIT>"))

(event `self.ReceiveTick`
  (params (DeltaSeconds :type "Float (single-precision)"))
  (bind _floatingnamecomp (`self.floatingNameComp`))
  (`SceneComponent.K2_SetWorldRotation` _floatingnamecomp (`KismetMathLibrary.MakeRotFromZX` (`KismetMathLibrary.GetUpVector` (struct)) (- (`SceneComponent.K2_GetComponentLocation` (`ChallengersCharacter.FollowCamera` (`self.PlayerREF`))) (`SceneComponent.K2_GetComponentLocation` _floatingnamecomp))) false false))

(event `self.Sphere.OnComponentBeginOverlap`
  (params (OverlappedComponent :type "PrimitiveComponent Object Reference") (OtherActor :type "Actor Object Reference") (OtherComp :type "PrimitiveComponent Object Reference") (OtherBodyIndex :type Integer) (bFromSweep :type Boolean) (SweepResult :type "HitResult Structure (by ref)"))
  (bind _asbp_challengers_character (cast `/Game/Yuchin/Blueprints/BP_ChallengersCharacter` OtherActor))
  (if (`self.HasAuthority` _asbp_challengers_character)
    (bind _outactors (`GameplayStatics.GetAllActorsOfClass` "/Game/BJK/BluePrints/BP_MainPlayerController.BP_MainPlayerController_C"))
    (`KismetSystemLibrary.PrintString` "host out")
    (for _array_element _outactors
      (`PlayerCameraManager.StartCameraFade` :`self` (`PlayerController.PlayerCameraManager` _array_element) :`ToAlpha` 1.0 :`Duration` 1.0 :`bShouldFadeAudio` true :`bHoldWhenFinished` true)
      (`KismetSystemLibrary.Delay` 1.0)
      (bind _asbp_our_game_instance (cast `/Game/Yuchin/Blueprints/BP_OurGameInstance` (`GameplayStatics.GetGameInstance`)))
      (set `OurGameInstance.bSLoading` true _asbp_our_game_instance)
      (`DestroySessionCallbackProxy.DestroySession` _array_element
        (:`then`
          (`GameplayStatics.OpenLevelBySoftObjectPtr` "/Game/Gothic_Cathedral/Maps/SingleMap.SingleMap"))))
    (else
      (bind _asmain_player_controller (cast `MainPlayerController` (`Pawn.GetController` _asbp_challengers_character)))
      (`KismetSystemLibrary.PrintString` "client")
      (`PlayerCameraManager.StartCameraFade` :`self` (`PlayerController.PlayerCameraManager` _asmain_player_controller) :`ToAlpha` 1.0 :`Duration` 1.0 :`bShouldFadeAudio` true :`bHoldWhenFinished` true)
      (`KismetSystemLibrary.Delay` 1.0)
      (`DestroySessionCallbackProxy.DestroySession` _asmain_player_controller
        (:`then`
          (bind _asbp_our_game_instance_2 (cast `/Game/Yuchin/Blueprints/BP_OurGameInstance` (`GameplayStatics.GetGameInstance`)))
          (set `OurGameInstance.bSLoading` true _asbp_our_game_instance_2)
          (`GameplayStatics.OpenLevelBySoftObjectPtr` "/Game/Gothic_Cathedral/Maps/SingleMap.SingleMap"))))))

(fn `UserConstructionScript`)