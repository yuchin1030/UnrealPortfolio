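; BP_MultiExitActor is a test actor that marks an exit with a floating "<EXIT>" label; it contains no exit logic.
; On BeginPlay it caches the BP_ChallengersCharacter and sets the text on the label's NameBillBoardWidget.
; Each Tick it billboards FloatingNameComp toward the player's FollowCamera, building the rotation from the camera direction and an up axis.
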(event `self.ReceiveBeginPlay`
  (bind _returnvalue (`GameplayStatics.GetActorOfClass` "/Game/Yuchin/Blueprints/BP_ChallengersCharacter.BP_ChallengersCharacter_C"))
  (set `self.Player` _returnvalue)
  (bind _asname_bill_board_widget (cast `NameBillBoardWidget` (`WidgetComponent.GetWidget` (`self.floatingNameComp`))))
  (`TextBlock.SetText` (`NameBillBoardWidget.name` _asname_bill_board_widget) "<EXIT>"))

(event `self.ReceiveTick`
  (params (DeltaSeconds :type "Float (single-precision)"))
  (bind _floatingnamecomp (`self.floatingNameComp`))
  (`SceneComponent.K2_SetWorldRotation` _floatingnamecomp (`KismetMathLibrary.MakeRotFromZX` (`KismetMathLibrary.GetUpVector` (struct)) (- (`SceneComponent.K2_GetComponentLocation` (`ChallengersCharacter.FollowCamera` (`self.Player`))) (`SceneComponent.K2_GetComponentLocation` _floatingnamecomp))) false false))

(fn `UserConstructionScript`)