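; BP_TestBulletShooter is a test actor that repeatedly spawns BP_BulletWindSlice bullets.
; On Tick, only the authority side adds delta time to an accumulator.
; Each time the accumulator passes a quarter second, it spawns a bullet at the Scene component's world transform and resets the timer.
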(event `self.ReceiveBeginPlay`)

(event `self.ReceiveTick`
  (params (DeltaSeconds :type "Float (single-precision)"))
  (`/Engine/EditorBlueprintResources/ActorMacros.Switch Has Authority`
    (:`Authority`
      (set `self.NewVar` (+ (`self.NewVar`) DeltaSeconds))
      (if (> (`self.NewVar`) 0.25)
        (`|SpawnActorFromClass` "/Game/CHR/Blueprints/Bullets/BP_BulletWindSlice.BP_BulletWindSlice_C" (`SceneComponent.K2_GetComponentToWorld` (`self.Scene`)) "Undefined" "MultiplyWithRoot" null null)
        (set `self.NewVar` 0.0)))))

(fn `UserConstructionScript`)