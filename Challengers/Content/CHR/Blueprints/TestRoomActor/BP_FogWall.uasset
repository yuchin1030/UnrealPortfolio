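; BP_FogWall is a wall actor that stays out of the camera's way and kills enemies that touch it.
; On BeginPlay it caches the player character and its own world X.
; Each Tick hides the Cube when the player's capsule and follow camera sit on opposite sides of that X plane.
; An enemy capsule entering the Box takes massive damage, effectively an instant kill.
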(event `self.ReceiveBeginPlay`
  (bind _returnvalue_x (`KismetMathLibrary.BreakVector` (`self.K2_GetActorLocation`)))
  (bind _asbp_challengers_character (cast `/Game/Yuchin/Blueprints/BP_ChallengersCharacter` (`GameplayStatics.GetPlayerCharacter` 0)))
  (set `self.As BP Challengers Character` _asbp_challengers_character)
  (set `self.WallX` _returnvalue_x))

(event `self.ReceiveTick`
  (params (DeltaSeconds :type "Float (single-precision)"))
  (bind _as_bp_challengers_character (`self.As BP Challengers Character`))
  (bind _wallx (`self.WallX`))
  (bind _wallx_2 (`self.WallX`))
  (bind _cube (`self.Cube`))
  (bind _returnvalue_x (`KismetMathLibrary.BreakVector` (`SceneComponent.K2_GetComponentLocation` (`Character.CapsuleComponent` _as_bp_challengers_character))))
  (bind _returnvalue_x_2 (`KismetMathLibrary.BreakVector` (`SceneComponent.K2_GetComponentLocation` (`ChallengersCharacter.FollowCamera` _as_bp_challengers_character))))
  (if (or (and (> _returnvalue_x _wallx) (< _returnvalue_x_2 _wallx)) (and (< _returnvalue_x _wallx_2) (> _returnvalue_x_2 _wallx_2)))
    (`SceneComponent.SetVisibility` _cube false false)
    (else
      (`SceneComponent.SetVisibility` _cube true false))))

(event `self.Box.OnComponentBeginOverlap`
  (params (OverlappedComponent :type "PrimitiveComponent Object Reference") (OtherActor :type "Actor Object Reference") (OtherComp :type "PrimitiveComponent Object Reference") (OtherBodyIndex :type Integer) (bFromSweep :type Boolean) (SweepResult :type "HitResult Structure (by ref)"))
  (bind _asbp_base_enemy (cast `/Game/CHR/Blueprints/BP_BaseEnemy` OtherActor))
  (cast `CapsuleComponent` OtherComp)
  (`GameplayStatics.ApplyDamage` _asbp_base_enemy 1000000.0))

(fn `UserConstructionScript`)