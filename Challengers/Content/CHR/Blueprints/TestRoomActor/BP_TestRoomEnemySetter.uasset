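; BP_TestRoomEnemySetter is a test-room marker prop with a floating "<장비 설정>" (equipment settings) name label; no setup logic is implemented here.
; On BeginPlay it sets the label, caches the player and assigns the mesh to RotatingMovement.
; A FlipFlop re-triggered by the Timeline's Finished pin alternates forward and reverse playback, bobbing the mesh endlessly.
; Tick billboards the label toward the player's follow camera.
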(event `self.ReceiveBeginPlay`
  (`|ExecutionSequence`
    (:`then_0`
      (bind _asname_bill_board_widget (cast `NameBillBoardWidget` (`WidgetComponent.GetWidget` (`self.floatingNameComp`))))
      (`TextBlock.SetText` (`NameBillBoardWidget.name` _asname_bill_board_widget) "<장비 설정>")
      (bind _returnvalue (`GameplayStatics.GetActorOfClass` "/Game/Yuchin/Blueprints/BP_ChallengersCharacter.BP_ChallengersCharacter_C"))
      (set `self.PlayerREF` _returnvalue)
      (bind _output_get (set `self.LowPos` (`SceneComponent.K2_GetComponentLocation` (`self.meshComp`))))
      (set `self.TopPos` (+ _output_get (0.0 0.0 20.0)))
      (`MovementComponent.SetUpdatedComponent` (`self.RotatingMovement`) (`self.meshComp`)))
    (:`then_1`
      (`/Engine/EditorBlueprintResources/StandardMacros.FlipFlop` :!label _label
        (:`A`
          (bind (_direction _value) (`Timeline|Timeline` :!via `PlayFromStart` :!label _label_2)
            (:`Update`
              (`SceneComponent.K2_SetWorldLocation` (`self.meshComp`) (`KismetMathLibrary.VLerp` (`self.LowPos`) (`self.TopPos`) _value) false false))
            (:`Finished`
              (goto _label))))
        (:`B`
          (goto _label_2 :!via `ReverseFromEnd`))))))

(event `self.ReceiveTick`
  (params (DeltaSeconds :type "Float (single-precision)"))
  (bind _floatingnamecomp (`self.floatingNameComp`))
  (`SceneComponent.K2_SetWorldRotation` _floatingnamecomp (`KismetMathLibrary.MakeRotFromZX` (`KismetMathLibrary.GetUpVector` (struct)) (- (`SceneComponent.K2_GetComponentLocation` (`ChallengersCharacter.FollowCamera` (`self.PlayerREF`))) (`SceneComponent.K2_GetComponentLocation` _floatingnamecomp))) false false))

(fn `UserConstructionScript`)