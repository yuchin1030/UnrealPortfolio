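; BP_TestExitMulti is an exit actor that sends the player to the SingleMap level when a challenger character enters its sphere.
; A floating name widget shows "<EXIT>" and turns every tick to face the follow camera of the first challenger found.
; On overlap, it fades the first player controller's camera and audio, waits a second, sets the game instance's SLoading flag, then opens the level.
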(event `self.ReceiveBeginPlay`
  (bind _returnvalue (`GameplayStatics.GetActorOfClass` "/Game/Yuchin/Blueprints/BP_ChallengersCharacter.BP_ChallengersCharacter_C"))
  (set `self.PlayerREF` _returnvalue)
  (bind _asname_bill_board_widget (cast `NameBillBoardWidget` (`WidgetComponent.GetWidget` (`self.floatingNameComp`))))
  (`TextBlock.SetText` (`NameBillBoardWidget.name` _asname_bill_board_widget) "<EXIT>"))

(event `self.ReceiveTick`
  (params (DeltaSeconds :type "Float (single-precision)"))
  (bind _floatingnamecomp (`self.floatingNameComp`))
  (bind _followcamera (`ChallengersCharacter.FollowCamera` (`self.PlayerREF`)))
  (`/Engine/EditorBlueprintResources/StandardMacros.IsValid` _followcamera
    (:`Is Valid`
      (`SceneComponent.K2_SetWorldRotation` _floatingnamecomp (`KismetMathLibrary.MakeRotFromZX` (`KismetMathLibrary.GetUpVector` (struct)) (- (`SceneComponent.K2_GetComponentLocation` _followcamera) (`SceneComponent.K2_GetComponentLocation` _floatingnamecomp))) false false))
    (:`Is Not Valid`
      (bind _returnvalue (`GameplayStatics.GetActorOfClass` "/Game/Yuchin/Blueprints/BP_ChallengersCharacter.BP_ChallengersCharacter_C"))
      (set `self.PlayerREF` _returnvalue))))

(event `self.Sphere.OnComponentBeginOverlap`
  (params (OverlappedComponent :type "PrimitiveComponent Object Reference") (OtherActor :type "Actor Object Reference") (OtherComp :type "PrimitiveComponent Object Reference") (OtherBodyIndex :type Integer) (bFromSweep :type Boolean) (SweepResult :type "HitResult Structure (by ref)"))
  (cast `/Game/Yuchin/Blueprints/BP_ChallengersCharacter` OtherActor)
  (`PlayerCameraManager.StartCameraFade` :`self` (`PlayerController.PlayerCameraManager` (`GameplayStatics.GetPlayerController` 0)) :`ToAlpha` 1.0 :`Duration` 1.0 :`bShouldFadeAudio` true :`bHoldWhenFinished` true)
  (`KismetSystemLibrary.Delay` 1.0)
  (bind _asbp_our_game_instance (cast `/Game/Yuchin/Blueprints/BP_OurGameInstance` (`GameplayStatics.GetGameInstance`)))
  (set `OurGameInstance.bSLoading` true _asbp_our_game_instance)
  (`GameplayStatics.OpenLevelBySoftObjectPtr` "/Game/Gothic_Cathedral/Maps/SingleMap.SingleMap"))

(fn `UserConstructionScript`)