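; Physics-driven projectile actor, filed with the MagicStaff assets, that explodes when it begins overlapping another actor.
; SetVelocity launches the mesh along the given view rotation, and an optional timer destroys the actor after a short delay.
; On overlap it spawns an explosion, then flings every movable overlapping component along one shared direction, from the mesh toward the triggering actor, before destroying itself.
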(event `self.ReceiveBeginPlay`
  (if (`self.isAutoSelfDestroy`)
    (`KismetSystemLibrary.Delay` 5.0)
    (`self.K2_DestroyActor`)))

(event `SetVelocity`
  (params (ForceLength :type "Float (double-precision)") (ViewRotation :type "Rotator Structure"))
  (`PrimitiveComponent.SetPhysicsLinearVelocity` (`self.Mesh`) (* (`KismetMathLibrary.Conv_RotatorToVector` ViewRotation) ForceLength) true "None"))

(event `self.ReceiveActorBeginOverlap`
  (params (OtherActor :type "Actor Object Reference"))
  (bind _returnvalue (`SceneComponent.K2_GetComponentLocation` (`self.Mesh`)))
  (`GameplayStatics.SpawnEmitterAtLocation` "/Game/Asset/EssentialAnimation/MagicStaff/Demo/Particles/P_Explosion.P_Explosion" _returnvalue)
  (for _array_element (`PrimitiveComponent.GetOverlappingComponents` (`self.Mesh`))
    (if (`|EnumEquality` (`SceneComponent.Mobility` _array_element) "Movable")
      (`PrimitiveComponent.SetPhysicsLinearVelocity` _array_element (* (`KismetMathLibrary.Normal` (- (`self.K2_GetActorLocation` OtherActor) _returnvalue)) 5000.0) false "None")))
  (`self.K2_DestroyActor`))

(fn `UserConstructionScript`)