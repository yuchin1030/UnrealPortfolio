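; BP_MovingShip is a ship actor that travels along a spline path in the level.
; On BeginPlay it finds the BP_ShipSpline actor and starts the MoveShip timeline, with play rate set from TimeToCompleteInSeconds.
; Each update maps the timeline alpha to a spline distance and sets location in world space, rotation in local space and a hardcoded scale.
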(event `self.ReceiveBeginPlay`
  (bind _returnvalue (`GameplayStatics.GetActorOfClass` "/Game/Yohan/BluePrints/BP_ShipSpline.BP_ShipSpline_C"))
  (set `self.ShipSpline` _returnvalue)
  (`self.MovingShip`))

(event `MovingShip`
  (bind _spline (`/Game/Yohan/BluePrints/BP_ShipSpline.Spline` (`self.ShipSpline`)))
  (`TimelineComponent.SetPlayRate` (`self.Move Ship`) (/ 1.0 (`self.Time To Complete(in Seconds)`)))
  (bind (_direction _movetrack) (`Timeline|Move Ship`)
    (:`Update`
      (bind _returnvalue (`KismetMathLibrary.Lerp` 0.0 (`SplineComponent.GetSplineLength` (`/Game/Yohan/BluePrints/BP_ShipSpline.Spline` (`self.ShipSpline`))) _movetrack))
      (`self.K2_SetActorTransform` (`KismetMathLibrary.MakeTransform` (`SplineComponent.GetLocationAtDistanceAlongSpline` _spline _returnvalue "World") (`SplineComponent.GetRotationAtDistanceAlongSpline` _spline _returnvalue "Local") (12.5 12.5 14.685))))))

(fn `UserConstructionScript`)