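; BP_DungeonEditCharacter is the character for dungeon editing, turning mouse clicks into enemy placement actions on its DungeonEditComponent.
; Right click shows the component's control widget; left click hides it, then calls SetEnemyLocation when nothing is being moved.
; While moving, left click confirms the selected enemy's position only on NavMesh, restoring collision, clearing its overlay material and deselecting it.
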(event `Key|LeftMouseButton`
  (params (Key :type "Key Structure"))
  (bind _dungeoneditcomponent (`self.dungeonEditComponent`))
  (bind _selectedenemy (`DungeonEditComponent.SelectedEnemy` _dungeoneditcomponent))
  (:`Pressed`
    (`|ExecutionSequence`
      (:`then_0`
        (`DungeonEditComponent.HideControlWidget` (`self.dungeonEditComponent`)))
      (:`then_1`
        (if (`DungeonEditComponent.bIsMoved` _dungeoneditcomponent)
          (`/Engine/EditorBlueprintResources/StandardMacros.IsValid` _selectedenemy
            (:`Is Valid`
              ;[1 1 1] 재배치할 때 NavMesh 위에 있다면..
              (bind _returnvalue (`DungeonEditComponent.IsEnemyOnNavMesh` _dungeoneditcomponent (`self.K2_GetActorLocation` _selectedenemy)))
              (if _returnvalue
                ;[1 1 1] 에너미 위치 고정
                (set `DungeonEditComponent.bIsObjectFixed` true _dungeoneditcomponent)
                (set `DungeonEditComponent.bIsMoved` false _dungeoneditcomponent)
                (`self.SetActorEnableCollision` _selectedenemy true)
                ;[1 1 1] 오버레이 없앰
                (`MeshComponent.SetOverlayMaterial` (`Character.Mesh` (`DungeonEditComponent.SelectedEnemy` _dungeoneditcomponent)) null)
                ;[1 1 1] Selected Enemy = null
                (set `DungeonEditComponent.SelectedEnemy` null _dungeoneditcomponent))))
          (else
            (`DungeonEditComponent.SetEnemyLocation` _dungeoneditcomponent)))))))

(event `Key|RightMouseButton`
  (params (Key :type "Key Structure"))
  (:`Pressed`
    (`DungeonEditComponent.ShowControlWidget` (`self.dungeonEditComponent`))))

(fn `UserConstructionScript`)