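; BP_Koopa_ball is a Koopa ball actor that drops into physics simulation and damages whatever it touches.
; Half a second after BeginPlay, it enables physics on its mesh and sphere components.
; Any actor overlapping its box component takes one point of damage.
; DestructBall is an empty event, and the hide-and-destroy node chain is unconnected, so the ball never removes itself here.
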(event `self.ReceiveBeginPlay`
  (`KismetSystemLibrary.Delay` 0.5)
  (`PrimitiveComponent.SetSimulatePhysics` (`self.meshComp`) true)
  (`PrimitiveComponent.SetSimulatePhysics` (`self.Sphere`) true))

(event `Destruct Ball`)

(event `self.boxComp.OnComponentBeginOverlap`
  (params (OverlappedComponent :type "PrimitiveComponent Object Reference") (OtherActor :type "Actor Object Reference") (OtherComp :type "PrimitiveComponent Object Reference") (OtherBodyIndex :type Integer) (bFromSweep :type Boolean) (SweepResult :type "HitResult Structure (by ref)"))
  (`GameplayStatics.ApplyDamage` OtherActor 1.0))

(fn `UserConstructionScript`)