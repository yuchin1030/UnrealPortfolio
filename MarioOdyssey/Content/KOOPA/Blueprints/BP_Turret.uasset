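; Koopa boss actor (named BP_Turret) whose attack cycle is gated by time windows on AnyTime.
; Tick feeds AnyTime and health to ABP_Turret, triggering timeline-driven jump teleports, mud effects, roars and fire, and resets the clock conditionally.
; Overlaps damage others during a timed window or spin.
; Damage lowers health, raises guard, knocks Koopa back at two thresholds with player reactions, and at zero destroys him, notifying the player.
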(event `self.ReceiveBeginPlay`)

(event `self.ReceiveTick`
  (params (DeltaSeconds :type "Float (single-precision)"))
  (bind _anytime (`self.anyTime`))
  (bind _fire1 (`self.fire1`))
  (`|ExecutionSequence`
    (:`then_0`
      (bind _asabp_turret_1 (cast `/Game/KOOPA/Koopa_skeletal/source/ABP_Turret1` (`SkeletalMeshComponent.GetAnimInstance` (`self.TurretMesh`))))
      (set `/Game/KOOPA/Koopa_skeletal/source/ABP_Turret1.ABPAnyTime` _anytime _asabp_turret_1)
      (set `/Game/KOOPA/Koopa_skeletal/source/ABP_Turret1.KoopaHealth` (`self.KoopaHealth`) _asabp_turret_1))
    (:`then_1`
      (if (and (> _anytime 5.0) (< _anytime 14.0))
        ;[1 1 1] 쿠파 점프하기
        (`|ExecutionSequence`
          (:`then_0`
            (if (not (`self.play`))
              (`KismetSystemLibrary.Delay` 0.5)
              (set `self.play` true)
              (bind (_direction _x _y _z) (`Timeline|Timeline_0` :!via `PlayFromStart`)
                (:`Update`
                  (`self.K2_TeleportTo` (`KismetMathLibrary.MakeVector` _x _y _z))
                  (`KismetSystemLibrary.Delay` 3.5)
                  (`NiagaraFunctionLibrary.SpawnSystemAtLocation` "/Game/A_Surface_Footstep/Niagara_FX/ParticleSystems/PSN_Mud_Surface.PSN_Mud_Surface" (-2040.0 1500.0 120.0))
                  (`|ExecutionSequence`
                    (:`then_0`
                      (`KismetSystemLibrary.Delay` 0.5)
                      (if (not (`self.play2`))
                        (`KismetSystemLibrary.Delay` 0.5)
                        (set `self.play2` true)
                        (bind (_direction_2 _x_2 _y_2 _z_2) (`Timeline|Timeline_1` :!via `PlayFromStart`)
                          (:`Update`
                            (`self.K2_TeleportTo` (`KismetMathLibrary.MakeVector` _x_2 _y_2 _z_2))
                            (`KismetSystemLibrary.Delay` 3.5)
                            (`NiagaraFunctionLibrary.SpawnSystemAtLocation` "/Game/A_Surface_Footstep/Niagara_FX/ParticleSystems/PSN_Mud_Surface.PSN_Mud_Surface" (-1110.0 440.0 120.0))
                            (set `self.playFire` false)))))))))))
        (elif (and (> _anytime 34.0) (< _anytime 35.0))
          (if (not (`self.play3`))
            (set `self.play3` true)
            (`KismetSystemLibrary.Delay` 0.5)
            (bind (_direction_3 _x_3 _y_3 _z_3) (`Timeline|Timeline` :!via `PlayFromStart`)
              (:`Update`
                (`self.K2_TeleportTo` (`KismetMathLibrary.MakeVector` _x_3 _y_3 _z_3))
                (`KismetSystemLibrary.Delay` 1.0)
                (set `self.play` false)
                (set `self.play2` false)))))))
    (:`then_2`
      (if (and (< _anytime 53.0) (> _anytime 43.0))
        ;[1 1 1] 쿠파 회전 불 스폰시키기, 주변에 불 켜기
        (`SceneComponent.SetVisibility` _fire1 true true)
        (`SceneComponent.SetVisibility` (`self.fire2`) true true)
        (`SceneComponent.SetVisibility` (`self.fire3`) true true)
        (`SceneComponent.SetVisibility` (`self.fire4`) true true)
        (`SceneComponent.SetVisibility` (`self.fire5`) true true)
        (`SceneComponent.SetVisibility` (`self.fire6`) true true)
        (`SceneComponent.SetVisibility` (`self.fire7`) true true)
        (`SceneComponent.SetVisibility` (`self.fire8`) true true)
        (if (not (`self.playFire`))
          (`|SpawnActorFromClass` "/Game/KOOPA/Blueprints/BP_fireTele1.BP_fireTele1_C" (`KismetMathLibrary.MakeTransform` (210.0 1350.0 90.0)) "Undefined" "MultiplyWithRoot" null null)
          (`|SpawnActorFromClass` "/Game/KOOPA/Blueprints/BP_fireTele.BP_fireTele_C" (`KismetMathLibrary.MakeTransform` (210.0 1350.0 90.0)) "Undefined" "MultiplyWithRoot" null null)
          (set `self.playFire` true)
          (set `self.play3` false))
        (elif (> _anytime 53.0)
          (`SceneComponent.SetVisibility` _fire1 false false)
          (`SceneComponent.SetVisibility` (`self.fire3`) false false)
          (`SceneComponent.SetVisibility` (`self.fire2`) false false)
          (`SceneComponent.SetVisibility` (`self.fire7`) false false)
          (`SceneComponent.SetVisibility` (`self.fire4`) false false)
          (`SceneComponent.SetVisibility` (`self.fire8`) false false)
          (`SceneComponent.SetVisibility` (`self.fire5`) false false)
          (`SceneComponent.SetVisibility` (`self.fire6`) false false))))
    (:`then_3`
      (if (or (and (> _anytime 38.0) (< _anytime 38.05)) (and (> _anytime 0.0) (< _anytime 0.05)))
        ;[1 1 1] 포효 나이아가라 스폰
        (`|SpawnActorFromClass` "/Game/KOOPA/Niagara/yelling.yelling_C" (`KismetMathLibrary.MakeTransform` (`SceneComponent.K2_GetComponentLocation` (`self.TurretMesh`))) "Undefined" "MultiplyWithRoot" null null)
        (`GameplayStatics.PlaySound2D` "/Game/Audio/Koopa/yelling_Cue.yelling_Cue" 1.0 1.0 0.0 null null)))
    (:`then_4`
      (bind _outactors (`GameplayStatics.GetAllActorsOfClass` "/Game/BP/BP_RealRecentCharacter.BP_RealRecentCharacter_C"))
      (if (and (not (`/Game/BP/BP_RealRecentCharacter.canThrow` (`|GetArrayItem` _outactors))) (> (`self.anyTime`) 54.0))
        (set `self.anyTime` 0.0)))))

(event `swing Hat`)

(event `self.ReceiveActorBeginOverlap`
  (params (OtherActor :type "Actor Object Reference")))

(event `self.Mario.OnComponentBeginOverlap`
  (params (OverlappedComponent :type "PrimitiveComponent Object Reference") (OtherActor :type "Actor Object Reference") (OtherComp :type "PrimitiveComponent Object Reference") (OtherBodyIndex :type Integer) (bFromSweep :type Boolean) (SweepResult :type "HitResult Structure (by ref)"))
  (bind _anytime (`self.anyTime`))
  (if (and (< _anytime 28.0) (> _anytime 19.0))
    (`GameplayStatics.ApplyDamage` OtherActor 1.0)))

(event `self.CupaCollision.OnComponentBeginOverlap`
  (params (OverlappedComponent :type "PrimitiveComponent Object Reference") (OtherActor :type "Actor Object Reference") (OtherComp :type "PrimitiveComponent Object Reference") (OtherBodyIndex :type Integer) (bFromSweep :type Boolean) (SweepResult :type "HitResult Structure (by ref)"))
  (cast `/Game/BP/BP_RealRecentCharacter` OtherActor)
  (set `self.isOverlappingCupa` true)
  (if (`self.isSpin`)
    (`GameplayStatics.ApplyDamage` OtherActor 1.0)))

(event `self.CupaCollision.OnComponentEndOverlap`
  (params (OverlappedComponent :type "PrimitiveComponent Object Reference") (OtherActor :type "Actor Object Reference") (OtherComp :type "PrimitiveComponent Object Reference") (OtherBodyIndex :type Integer))
  (cast `/Game/BP/BP_RealRecentCharacter` OtherActor)
  (set `self.isOverlappingCupa` false))

(event `Damage`
  (bind _koopahealth (`self.KoopaHealth`))
  (`|ExecutionSequence`
    (:`then_0`
      (bind _output_get (set `self.KoopaHealth` (- (`self.KoopaHealth`) 1)))
      (`KismetSystemLibrary.PrintString` (`KismetStringLibrary.Conv_IntToString` _output_get))
      (`NiagaraFunctionLibrary.SpawnSystemAtLocation` "/Game/A_Surface_Footstep/Niagara_FX/ParticleSystems/PSN_General1_Surface.PSN_General1_Surface" (`SceneComponent.GetForwardVector` (`self.TurretMesh`)))
      (if (or (== _koopahealth 29) (== _koopahealth 14))
        (`|ExecutionSequence`
          (:`then_0`
            (bind (_direction _back) (`Timeline|CupaBack` :!via `PlayFromStart`)
              (:`Update`
                (`SceneComponent.K2_SetRelativeLocation` (`self.TurretMesh`) (`KismetMathLibrary.MakeVector` 0.0 _back) false false))))
          (:`then_1`
            (bind _asbp_real_recent_character (cast `/Game/BP/BP_RealRecentCharacter` (`GameplayStatics.GetPlayerCharacter` 0)))
            (`/Game/BP/BP_RealRecentCharacter.TTiYYoung` _asbp_real_recent_character)
            (`KismetSystemLibrary.Delay` 1.0)
            (`/Game/BP/BP_RealRecentCharacter.TakeOffHat` _asbp_real_recent_character)))
        (elif (<= (`self.KoopaHealth`) 0)
          (`KismetSystemLibrary.Delay` 3.0)
          (`self.K2_DestroyActor`)
          (bind _asbp_real_recent_character_2 (cast `/Game/BP/BP_RealRecentCharacter` (`GameplayStatics.GetPlayerCharacter` 0)))
          (set `/Game/BP/BP_RealRecentCharacter.isCupaAlive` false _asbp_real_recent_character_2))))
    (:`then_1`
      (set `self.KoopaGuard` true))))

(fn `UserConstructionScript`)