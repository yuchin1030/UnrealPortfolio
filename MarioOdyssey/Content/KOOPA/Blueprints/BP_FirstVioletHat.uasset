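; BP_FirstVioletHat is a hat hazard that damages whatever overlaps it and can be destroyed by Mario's thrown cap.
; Its box overlap applies damage and clears OverlapMario, then starts a delay that leads nowhere.
; The same overlap checks for BP_MarioThrowingCap, stops the cap's movement and destroys the hat.
; A random roll, printed to screen, spawns a BP_RealStamina pickup when it reaches Rate.
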(event `self.boxComp.OnComponentBeginOverlap`
  (params (OverlappedComponent :type "PrimitiveComponent Object Reference") (OtherActor :type "Actor Object Reference") (OtherComp :type "PrimitiveComponent Object Reference") (OtherBodyIndex :type Integer) (bFromSweep :type Boolean) (SweepResult :type "HitResult Structure (by ref)"))
  (`|ExecutionSequence`
    (:`then_0`
      (`GameplayStatics.ApplyDamage` OtherActor 1.0) ; 닿으면 damage
      (set `self.overlapMario` false)
      (`KismetSystemLibrary.Delay` 3.0))
    (:`then_1`
      (bind _asbp_mario_throwing_cap (cast `/Game/BP/BP_MarioThrowingCap` OtherActor)) ; 모자 throw하면 모자 죽임 + 아이템 랜덤 생성
      (`MovementComponent.StopMovementImmediately` (`/Game/BP/BP_MarioThrowingCap.ProjectileMovement` _asbp_mario_throwing_cap))
      (bind _output_get (set `self.num` (`KismetMathLibrary.RandomIntegerInRange` 1 100)))
      (`KismetSystemLibrary.PrintString` (`KismetStringLibrary.Conv_IntToString` _output_get))
      (if (>= _output_get (`self.rate`))
        (`|SpawnActorFromClass` "/Game/BP/BP_RealStamina.BP_RealStamina_C" (`self.GetTransform`) "Undefined" "MultiplyWithRoot" null null)
        (`self.K2_DestroyActor`)
        (else
          (`self.K2_DestroyActor`))))))

(fn `UserConstructionScript`)