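; BP_fireTele1 is a short-lived, spinning fire hazard that damages and ignites the player character on contact.
; It removes itself after a fixed lifespan and turns steadily around yaw every tick, at a frame-rate-dependent rate.
; Box overlap with BP_RealRecentCharacter sets its ImFire flag, applies damage, puts an overlay material on its mesh and activates its NSBlood effect.
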(event `self.ReceiveBeginPlay`
  (`self.SetLifeSpan` 10.0))

(event `self.ReceiveTick`
  (params (DeltaSeconds :type "Float (single-precision)"))
  (bind (_returnvalue_roll _returnvalue_pitch _returnvalue_yaw) (`KismetMathLibrary.BreakRotator` (`self.K2_GetActorRotation`)))
  (`self.K2_SetActorRotation` (`KismetMathLibrary.MakeRotator` _returnvalue_roll _returnvalue_pitch (+ _returnvalue_yaw -1.0))))

(event `self.Box.OnComponentBeginOverlap`
  (params (OverlappedComponent :type "PrimitiveComponent Object Reference") (OtherActor :type "Actor Object Reference") (OtherComp :type "PrimitiveComponent Object Reference") (OtherBodyIndex :type Integer) (bFromSweep :type Boolean) (SweepResult :type "HitResult Structure (by ref)"))
  (bind _asbp_real_recent_character (cast `/Game/BP/BP_RealRecentCharacter` OtherActor))
  (`|ExecutionSequence`
    (:`then_0`
      (set `/Game/BP/BP_RealRecentCharacter.ImFire` true _asbp_real_recent_character)
      (`GameplayStatics.ApplyDamage` OtherActor 1.0))
    (:`then_1`
      (`MeshComponent.SetOverlayMaterial` (`Character.Mesh` _asbp_real_recent_character) "/Game/YCAsset/M_Overlay.M_Overlay")
      (`ActorComponent.Activate` (`/Game/BP/BP_RealRecentCharacter.NS_Blood` _asbp_real_recent_character) false))))

(fn `UserConstructionScript`)