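; BP_DestroyingWhiteHat is a white hat actor that flies off behind Mario and bursts when the character's CanDestroyHat flag is set.
; BeginPlay caches the BP_RealRecentCharacter reference.
; While flagged, Tick moves the hat backward and up relative to Mario, activates RotatingMovement, and turns it once to face him via RotateDir.
; A half-second Delay then spawns the NS_Pung1 Niagara effect and destroys the actor.
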(event `self.ReceiveBeginPlay`
  (bind _outactors (`GameplayStatics.GetAllActorsOfClass` "/Game/BP/BP_RealRecentCharacter.BP_RealRecentCharacter_C"))
  (set `self.CharacterVar` (`|GetArrayItem` _outactors)))

(event `self.ReceiveTick`
  (params (DeltaSeconds :type "Float (single-precision)"))
  (bind _destroyhatspeed (`self.DestroyHatSpeed`))
  (if (`/Game/BP/BP_RealRecentCharacter.CanDestroyHat` (`self.CharacterVar`))
    (`|ExecutionSequence`
      (:`then_0`
        (`self.K2_SetActorLocation` (+ (`self.K2_GetActorLocation`) (* (`KismetMathLibrary.Normal` (* (`self.GetActorForwardVector` (`self.CharacterVar`)) -1.0) 1.0) _destroyhatspeed DeltaSeconds) (* (`KismetMathLibrary.Normal` (`self.GetActorUpVector` (`self.CharacterVar`)) 1.0) _destroyhatspeed DeltaSeconds))) ; 마리오 뒤방향으로 날라가게끔
        (`KismetSystemLibrary.Delay` 0.5)
        (`NiagaraFunctionLibrary.SpawnSystemAtLocation` "/Game/VFX/NS_Pung1.NS_Pung1" (`self.K2_GetActorLocation`) (`self.K2_GetActorRotation`))
        (`self.K2_DestroyActor`))
      (:`then_1`
        (`ActorComponent.Activate` (`self.RotatingMovement`) false) ; 회전하면서 날라가게끔
      )
      (:`then_2`
        (`/Engine/EditorBlueprintResources/StandardMacros.DoOnce` false
          (:`Completed`
            (`self.RotateDir`)))))))

(event `RotateDir`
  (bind (_returnvalue_roll _returnvalue_pitch _returnvalue_yaw) (`KismetMathLibrary.BreakRotator` (`KismetMathLibrary.MakeRotFromZX` (`self.GetActorUpVector`) (- (`self.K2_GetActorLocation` (`self.CharacterVar`)) (`self.K2_GetActorLocation`)))))
  (`self.K2_SetActorRotation` (`KismetMathLibrary.MakeRotator` _returnvalue_roll _returnvalue_pitch _returnvalue_yaw)) ; 항상 마리오 뒤로 마리아를 바라보면서 모자가 날라가게끔 돌려줌
)

(fn `UserConstructionScript`)