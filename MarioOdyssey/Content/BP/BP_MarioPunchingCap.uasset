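; BP_MarioPunchingCap is a Koopa hat actor that damages whatever overlaps it until it gets knocked back and becomes wearable.
; CupaHatRotate starts a Timeline that pitches the hat and sets CanWearHat, while UpdateInterp builds three arc points leading away from the player.
; Tick lerps through those points over two seconds.
; Overlap events track whether BP_RealRecentCharacter is touching the hat.
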(event `self.ReceiveBeginPlay`
  (bind (_returnvalue_roll _returnvalue_pitch) (`KismetMathLibrary.BreakRotator` (`self.K2_GetActorRotation`)))
  (`|ExecutionSequence`
    (:`then_0`
      (bind _outactors (`GameplayStatics.GetAllActorsOfClass` "/Game/BP/BP_MarioThrowingCap.BP_MarioThrowingCap_C"))
      (set `self.ThrowCapVar` (`|GetArrayItem` _outactors))
      (set `self.NewRotY` _returnvalue_pitch))
    (:`then_1`
      (bind _outactors_2 (`GameplayStatics.GetAllActorsOfClass` "/Game/BP/BP_RealRecentCharacter.BP_RealRecentCharacter_C"))
      (set `self.CharacterVar` (`|GetArrayItem` _outactors_2)))))

(event `self.CupaHatCollision.OnComponentBeginOverlap`
  (params (OverlappedComponent :type "PrimitiveComponent Object Reference") (OtherActor :type "Actor Object Reference") (OtherComp :type "PrimitiveComponent Object Reference") (OtherBodyIndex :type Integer) (bFromSweep :type Boolean) (SweepResult :type "HitResult Structure (by ref)"))
  (`|ExecutionSequence`
    (:`then_0`
      (if (not (`self.CanWearHat`))
        (`GameplayStatics.ApplyDamage` OtherActor 1.0)))
    (:`then_1`
      (cast `/Game/BP/BP_RealRecentCharacter` OtherActor)
      (set `self.isOverlappingHat` true)
      (`KismetSystemLibrary.PrintString` "yes overlap"))))

(event `self.CupaHatCollision.OnComponentEndOverlap`
  (params (OverlappedComponent :type "PrimitiveComponent Object Reference") (OtherActor :type "Actor Object Reference") (OtherComp :type "PrimitiveComponent Object Reference") (OtherBodyIndex :type Integer))
  (cast `/Game/BP/BP_RealRecentCharacter` OtherActor)
  (set `self.isOverlappingHat` false)
  (`KismetSystemLibrary.PrintString` "no overlap"))

(event `CupaHatRotate`
  (set `self.StopRot` true)
  (`self.UpdateInterp`)
  (bind (_direction _newtrack_0) (`Timeline|Timeline`)
    (:`Update`
      (`self.K2_SetActorRotation` (`KismetMathLibrary.MakeRotator` 0.0 _newtrack_0))
      (set `self.CanWearHat` true)
      (`KismetSystemLibrary.PrintString` "모자 쓸 수 있는 상태 Ready"))))

(event `UpdateInterp`
  (bind _test (`self.Test`))
  (bind (_returnvalue_x _returnvalue_y _returnvalue_z) (`KismetMathLibrary.BreakVector` (`SceneComponent.K2_GetComponentLocation` (`self.CupaHatCollision`))))
  (bind _asbp_real_recent_character (cast `/Game/BP/BP_RealRecentCharacter` (`GameplayStatics.GetPlayerCharacter` 0)))
  (bind _returnvalue (- (`SceneComponent.K2_GetComponentLocation` (`self.CupaHatCollision`)) (`self.K2_GetActorLocation` _asbp_real_recent_character)))
  (set `self.moveDir` (`KismetMathLibrary.Normal` _returnvalue))
  (`KismetArrayLibrary.Array_Set` _test 0 (+ (* _returnvalue_x (`self.GetActorForwardVector`)) (* _returnvalue_y (`self.GetActorRightVector`)) (* _returnvalue_z (`self.GetActorUpVector`))))
  (bind (_returnvalue_x_2 _returnvalue_y_2) (`KismetMathLibrary.BreakVector` (+ (`SceneComponent.K2_GetComponentLocation` (`self.CupaHatCollision`)) _returnvalue)))
  (`KismetArrayLibrary.Array_Set` _test 1 (+ (* _returnvalue_x_2 (`self.GetActorForwardVector`)) (* _returnvalue_y_2 (`self.GetActorRightVector`)) (0.0 0.0 500.0)))
  (`KismetArrayLibrary.Array_Set` _test 2 (+ (* _returnvalue_x_2 (`self.GetActorForwardVector`)) (* _returnvalue_y_2 (`self.GetActorRightVector`)) (* _returnvalue_z (`self.GetActorUpVector`))))
  (set `self.Shoot` true))

(event `self.ReceiveTick`
  (params (DeltaSeconds :type "Float (single-precision)"))
  (bind _test (`self.Test`))
  (bind _test_2 (`self.Test`))
  (if (`self.Shoot`)
    (bind _output_get (set `self.Delta` (`KismetMathLibrary.FClamp` (+ DeltaSeconds (`self.Delta`)) 0.0 2.0)))
    (if (<= _output_get 1.0)
      (`self.K2_SetActorLocation` (`KismetMathLibrary.VLerp` (`|GetArrayItem` _test) (`|GetArrayItem` _test 1) _output_get))
      (else
        (bind _returnvalue (- _output_get 1.0))
        (`self.K2_SetActorLocation` (`KismetMathLibrary.VLerp` (`|GetArrayItem` _test_2 1) (`|GetArrayItem` _test_2 2) _returnvalue))
        (if (>= _returnvalue 1.0)
          (set `self.Shoot` false))))))

(fn `UserConstructionScript`)