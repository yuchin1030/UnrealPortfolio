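; Mario's thrown cap actor, which flies out via projectile movement and can return to the player character.
; Tick stops the projectile immediately when the level's BP_WhiteHat is throwing, otherwise after a 0.2-second delay.
; ReturnToPlayer runs once, moving the cap to the player's mesh, re-showing the worn cap and destroying itself.
; A separate Heal event raises clamped Mario HP and updates the player's HP UI.
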(event `self.ReceiveBeginPlay`
  (bind _outactors (`GameplayStatics.GetAllActorsOfClass` "/Game/BP/BP_RealRecentCharacter.BP_RealRecentCharacter_C"))
  (set `self.CharacterVar` (`|GetArrayItem` _outactors))
  (bind _outactors_2 (`GameplayStatics.GetAllActorsOfClass` "/Game/KOOPA/Blueprints/BP_WhiteHat.BP_WhiteHat_C"))
  (set `self.PunchCapVar` (`|GetArrayItem` _outactors_2)))

(event `self.ReceiveTick`
  (params (DeltaSeconds :type "Float (single-precision)"))
  (bind _punchcapvar (`self.PunchCapVar`))
  (`/Engine/EditorBlueprintResources/StandardMacros.IsValid` _punchcapvar
    (:`Is Valid`
      (if (`/Game/KOOPA/Blueprints/BP_WhiteHat.isThrowingCap` _punchcapvar)
        (`MovementComponent.StopMovementImmediately` (`self.ProjectileMovement`)) ; 쿠파가 던진 모자 enemy에 맞으면 그 자리에서 throw stop
        (else
          (`KismetSystemLibrary.Delay` 0.2)
          (`MovementComponent.StopMovementImmediately` (`self.ProjectileMovement`)))))))

(event `ReturnToPlayer`
  ;[1 1 1] 모자 날리고 되돌아오기
  (`/Engine/EditorBlueprintResources/StandardMacros.DoOnce` false
    (:`Completed`
      (bind _asbp_real_recent_character (cast `/Game/BP/BP_RealRecentCharacter` (`GameplayStatics.GetPlayerCharacter` 0)))
      (bind (_returnvalue_location _returnvalue_rotation) (`KismetMathLibrary.BreakTransform` (`SceneComponent.K2_GetComponentToWorld` (`Character.Mesh` _asbp_real_recent_character))))
      (`KismetSystemLibrary.MoveComponentTo` (`self.DefaultSceneRoot`) _returnvalue_location _returnvalue_rotation)
      (`SceneComponent.SetVisibility` (`/Game/BP/BP_RealRecentCharacter.Cap` _asbp_real_recent_character) true false)
      (`self.K2_DestroyActor`))))

(event `Heal`
  (set `self.MarioHp` (`KismetMathLibrary.FClamp` (+ (`self.MarioHP`) 1.0) 0.0 6.0))
  (bind _asbp_real_recent_character (cast `/Game/BP/BP_RealRecentCharacter` (`GameplayStatics.GetPlayerCharacter` 0)))
  (`/Game/UI/MarioHp.PlusHp` (`/Game/BP/BP_RealRecentCharacter.UI_MarioHP` _asbp_real_recent_character) 0.0))

(fn `UserConstructionScript`)