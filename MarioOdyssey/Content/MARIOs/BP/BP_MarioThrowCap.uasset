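; Mario's thrown cap actor, which returns to the player and also carries a heal event.
; ReturnToPlayer moves the root to the player's mesh transform once, shows the character's own Cap again and destroys this actor.
; Heal raises a clamped MarioHp and updates the HP widget through BP_ThirdPersonCharacter, whereas the return casts to BP_RealRecentCharacter.
; BeginPlay caches character and PunchCap references, but line-trace and Cupa-hat stop logic is left disconnected.
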(event `self.ReceiveBeginPlay`
  (bind _outactors (`GameplayStatics.GetAllActorsOfClass` "/Game/BP/BP_RealRecentCharacter.BP_RealRecentCharacter_C"))
  (set `self.CharacterVar` (`|GetArrayItem` _outactors))
  (bind _outactors_2 (`GameplayStatics.GetAllActorsOfClass` "/Game/MARIOs/BP/PunchCap.PunchCap_C"))
  (set `self.PunchCap Var` (`|GetArrayItem` _outactors_2)))

(event `self.ReceiveTick`
  (params (DeltaSeconds :type "Float (single-precision)")))

(event `ReturnToPlayer`
  ;[1 1 1] 모자 날리고 되돌아오기
  (`/Engine/EditorBlueprintResources/StandardMacros.DoOnce` false
    (:`Completed`
      (bind _asbp_real_recent_character (cast `/Game/BP/BP_RealRecentCharacter` (`GameplayStatics.GetPlayerCharacter` 0)))
      (bind (_returnvalue_location _returnvalue_rotation) (`KismetMathLibrary.BreakTransform` (`SceneComponent.K2_GetComponentToWorld` (`Character.Mesh` _asbp_real_recent_character))))
      (`KismetSystemLibrary.MoveComponentTo` (`self.DefaultSceneRoot`) _returnvalue_location _returnvalue_rotation)
      (`SceneComponent.SetVisibility` (`/Game/BP/BP_RealRecentCharacter.Cap` _asbp_real_recent_character) true false)
      (`self.K2_DestroyActor`))))

(event `Heal`
  (set `self.MarioHp` (`KismetMathLibrary.FClamp` (+ (`self.MarioHP`) 1.0) 0.0 6.0))
  (bind _asbp_third_person_character (cast `/Game/ThirdPerson/Blueprints/BP_ThirdPersonCharacter` (`GameplayStatics.GetPlayerCharacter` 0)))
  (`/Game/UI/MarioHp.PlusHp` (`/Game/ThirdPerson/Blueprints/BP_ThirdPersonCharacter.UI_MarioHp` _asbp_third_person_character) 0.0))

(fn `UserConstructionScript`)